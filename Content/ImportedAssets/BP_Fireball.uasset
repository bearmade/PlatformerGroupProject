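; 2D side-scroller fireball hazard that repeatedly rises and falls vertically, hurting the player on overlap.
; After a random start delay, Tick detaches a tile sprite in world space and runs a MoveState machine: up, down, random pause, with matching flame flipbooks.
; Travel counts ticks, so motion is frame-rate dependent.
; Overlap applies SubHealth and knockback, then a timer restores damage and player vulnerability.
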(event Custom|CustomEvent_1
  (Variables|Default|SetcanDamage true)
  (Variables|/Game/Player/BP_2DSidescrollerCharacter.BP_2DSidescrollerCharacter_C|SetcanBeHurt (stale Collision|EventActorBeginOverlap _asbp_2dsidescroller_character) true))

(event EventBeginPlay
  (Variables|Default|Settimer (Math|Random|RandomIntegerinRange 3 10))
  (Utilities|FlowControl|Delay (Math|Conversions|ToFloat(Integer) (Variables|Default|Gettimer)))
  (Variables|Default|SetstartFire true)
  (Variables|Default|SetmovingUP true)
  (Variables|Default|SetcanDamage true)
  (Variables|Default|SetmoveState 0))

(event Collision|EventActorBeginOverlap
  (params (OtherActor :type Actor%20Object%20Reference))
  (if (Variables|Default|GetcanDamage)
    (bind _asbp_2dsidescroller_character (Utilities|Casting|CastToBP_2DSidescrollerCharacter (Game|GetPlayerCharacter 0)))
    (if (Collision|IsOverlappingActor _asbp_2dsidescroller_character :!class /Script/Engine.Actor)
      (Default|SubHealth _asbp_2dsidescroller_character -5)
      (Default|KnockBack _asbp_2dsidescroller_character)
      (Variables|/Game/Player/BP_2DSidescrollerCharacter.BP_2DSidescrollerCharacter_C|SetcanBeHurt _asbp_2dsidescroller_character false)
      (Variables|Default|SetcanDamage false)
      (Utilities|Time|SetTimerbyEvent (delegate Custom|CustomEvent_1) 2.0))))

(event EventTick
  (params (DeltaSeconds :type Float%20%28single-precision%29))
  (bind _speed (Variables|Default|Getspeed))
  (if (Variables|Default|GetstartFire)
    (Transformation|DetachFromComponent (Variables|Default|GetTileSet_Sprite_6) "KeepWorld" "KeepRelative" "KeepRelative" true)
    (switch int (Variables|Default|GetmoveState)
      (:0
        (Sprite|SetFlipbook (Variables|Default|GetFB_FLame) "/Game/ImportedAssets/FB_FlameUP.FB_FlameUP")
        (Variables|Default|SetdistTraveled (+ (Variables|Default|GetdistTraveled) 1))
        (Transformation|SetActorLocation (+ (Transformation|GetActorLocation) (Math|Vector|MakeVector 0.0 0.0 _speed)) false false)
        (if (> (Variables|Default|GetdistTraveled) (Variables|Default|Getdistance))
          (Variables|Default|SetdistTraveled 0)
          (Variables|Default|SetmoveState 1)
          (Variables|Default|SetmovingUP false)))
      (:1
        (Sprite|SetFlipbook (Variables|Default|GetFB_FLame) "/Game/ImportedAssets/FB_FLameDown.FB_FLameDown")
        (Variables|Default|SetdistTraveled (+ (Variables|Default|GetdistTraveled) 1))
        (Transformation|SetActorLocation (+ (Transformation|GetActorLocation) (Math|Vector|MakeVector 0.0 0.0 (* _speed -1.0))) false false)
        (if (> (Variables|Default|GetdistTraveled) (Variables|Default|Getdistance))
          (Variables|Default|SetdistTraveled 0)
          (Variables|Default|SetmoveState 2)
          (Variables|Default|SetmovingUP true)))
      (:2
        (Utilities|FlowControl|Delay (Math|Random|RandomFloatinRange 0.5 5.0))
        (Variables|Default|SetmoveState 0)))))

(fn ConstructionScript)