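; Spike hazard that hurts and knocks back the 2D sidescroller player character on contact.
; Overlap start calls SubHealth and KnockBack, clears the character's CanBeHurt, and disables spike damage for a three-second timer.
; Tick repeats the hit while the player stays overlapping and damage is re-enabled, without clearing CanBeHurt.
; The timer re-enables damage and restores CanBeHurt through the overlap event's cast reference.
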(event Custom|damageDelay
  (Variables|Default|SetcanDamage true)
  (Variables|/Game/Player/BP_2DSidescrollerCharacter.BP_2DSidescrollerCharacter_C|SetcanBeHurt (stale Collision|EventActorBeginOverlap _asbp_2dsidescroller_character) true))

(event EventBeginPlay
  (Variables|Default|SetcanDamage true))

(event Collision|EventActorBeginOverlap
  (params (OtherActor :type Actor%20Object%20Reference))
  (if (Variables|Default|GetcanDamage)
    (bind _asbp_2dsidescroller_character (Utilities|Casting|CastToBP_2DSidescrollerCharacter OtherActor))
    (Default|SubHealth _asbp_2dsidescroller_character -5)
    (Default|KnockBack _asbp_2dsidescroller_character)
    (Variables|/Game/Player/BP_2DSidescrollerCharacter.BP_2DSidescrollerCharacter_C|SetcanBeHurt _asbp_2dsidescroller_character false)
    (Variables|Default|SetcanDamage false)
    (Utilities|Time|SetTimerbyEvent (delegate Custom|damageDelay) 3.0)))

(event EventTick
  (params (DeltaSeconds :type Float%20%28single-precision%29))
  (if (Variables|Default|GetcanDamage)
    (bind _asbp_2dsidescroller_character (Utilities|Casting|CastToBP_2DSidescrollerCharacter (Game|GetPlayerCharacter 0)))
    (if (Collision|IsOverlappingActor _asbp_2dsidescroller_character :!class /Script/Engine.Actor)
      (Default|SubHealth _asbp_2dsidescroller_character -5)
      (Default|KnockBack _asbp_2dsidescroller_character)
      (Variables|Default|SetcanDamage false)
      (Utilities|Time|SetTimerbyEvent (delegate Custom|damageDelay) 3.0))))

(fn ConstructionScript)