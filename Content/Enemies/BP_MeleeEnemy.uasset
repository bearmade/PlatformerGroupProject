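; Melee enemy for a 2D sidescroller that damages the player at close range, built on a parent enemy class.
; Attack starts a looping timer that checks HitBox against Target, plays the attack flipbook and applies damage, with a short timer restoring idle.
; Parent Tick is skipped while attacking.
; When the player leaves AttackCollision, re-setting the check timer with zero time cancels the loop and Following is re-enabled.
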(event OnComponentEndOverlap(AttackCollision)
  (params (OverlappedComponent :type Primitive%20Component%20Object%20Reference) (OtherActor :type Actor%20Object%20Reference) (OtherComp :type Primitive%20Component%20Object%20Reference) (OtherBodyIndex :type Integer))
  (Utilities|Casting|CastToBP_2DSidescrollerCharacter OtherActor)
  (Utilities|Time|SetTimerbyEvent (delegate Custom|CheckForHit) 0.0)
  (Variables|Default|SetbFollowing true))

(event Custom|CheckForHit
  (Variables|Default|SetisAttacking false)
  (if (Collision|IsOverlappingActor (Variables|Default|GetHitBox) (Variables|Default|GetTarget) :!class /Script/Engine.PrimitiveComponent)
    (Variables|Default|SetisAttacking true)
    (Sprite|SetFlipbook (Variables|Default|GetSprite) "/Game/Enemies/Enemy_Attack_Flipbook.Enemy_Attack_Flipbook")
    (Utilities|Time|SetTimerbyEvent (delegate Custom|StopAttacking) 0.2)
    (Utilities|Casting|CastToBP_2DSidescrollerCharacter (Variables|Default|GetTarget))
    (Game|Damage|ApplyDamage (Game|GetPlayerCharacter 0) 5.0 0 0)))

(event Custom|StopAttacking
  (Variables|Default|SetisAttacking false)
  (Sprite|SetFlipbook (Variables|Default|GetSprite) "/Game/Enemies/Enemy_Idle_Flipbook.Enemy_Idle_Flipbook"))

(event EventBeginPlay
  (|CallParentFunction) ; This node is disabled and will not be called.\nDrag off pins to build functionality.
)

(event Collision|EventActorBeginOverlap
  (params (OtherActor :type Actor%20Object%20Reference))
  (|CallParentFunction OtherActor) ; This node is disabled and will not be called.\nDrag off pins to build functionality.
)

(event EventTick
  (params (DeltaSeconds :type Float%20%28single-precision%29))
  (if (not (Variables|Default|GetisAttacking))
    (|CallParentFunction DeltaSeconds)))

(event EventAttack
  (CallFunction|CheckforHit)
  (Utilities|Time|SetTimerbyEvent (delegate Custom|CheckForHit) 0.5 true))

(fn ConstructionScript
  (|CallParentFunction))