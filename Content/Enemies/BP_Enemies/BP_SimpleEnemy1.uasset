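; Mushroom enemy for the 2D sidescroller that walks forward every tick and turns around when its WallDetection volume overlaps something.
; FollowCollision stores the player as target and nudges movement toward it once, while AttackCollision only toggles the Following flag, with no attack.
; The continuous chase, velocity-based facing and idle/run flipbook update are disconnected, so they never run.
; Follow and wall overlaps print debug strings.
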(event OnComponentBeginOverlap(FollowCollision)
  (params (OverlappedComponent :type Primitive%20Component%20Object%20Reference) (OtherActor :type Actor%20Object%20Reference) (OtherComp :type Primitive%20Component%20Object%20Reference) (OtherBodyIndex :type Integer) (bFromSweep :type Boolean) (SweepResult :type Hit%20Result%20Structure%20%28by%20ref%29))
  ;[0.5776 0.5841 0.2502] Following 2D Character
  (bind _asbp_2dsidescroller_character (Utilities|Casting|CastToBP_2DSidescrollerCharacter OtherActor))
  (Variables|Default|SetTarget _asbp_2dsidescroller_character)
  (Variables|Default|SetbFollowing true)
  (CallFunction|MovetoTarget)
  (Development|PrintString "Follow"))

(event OnComponentEndOverlap(FollowCollision)
  (params (OverlappedComponent :type Primitive%20Component%20Object%20Reference) (OtherActor :type Actor%20Object%20Reference) (OtherComp :type Primitive%20Component%20Object%20Reference) (OtherBodyIndex :type Integer))
  ;[0.5776 0.5841 0.2502] Following 2D Character
  (Utilities|Casting|CastToBP_2DSidescrollerCharacter OtherActor)
  (Variables|Default|SetbFollowing false))

(event OnComponentBeginOverlap(AttackCollision)
  (params (OverlappedComponent :type Primitive%20Component%20Object%20Reference) (OtherActor :type Actor%20Object%20Reference) (OtherComp :type Primitive%20Component%20Object%20Reference) (OtherBodyIndex :type Integer) (bFromSweep :type Boolean) (SweepResult :type Hit%20Result%20Structure%20%28by%20ref%29))
  (bind _target (Variables|Default|GetTarget))
  ;[0.5651 0.07505 0.07505] Attacking 2D Character
  (if (== OtherActor _target)
    (Utilities|Casting|CastToBP_2DSidescrollerCharacter _target)
    (Variables|Default|SetbFollowing false)))

(event OnComponentEndOverlap(AttackCollision)
  (params (OverlappedComponent :type Primitive%20Component%20Object%20Reference) (OtherActor :type Actor%20Object%20Reference) (OtherComp :type Primitive%20Component%20Object%20Reference) (OtherBodyIndex :type Integer))
  ;[0.5651 0.07505 0.07505] Attacking 2D Character
  (if (== OtherActor (Variables|Default|GetTarget))
    (Variables|Default|SetbFollowing true)))

(event OnComponentBeginOverlap(WallDetection)
  (params (OverlappedComponent :type Primitive%20Component%20Object%20Reference) (OtherActor :type Actor%20Object%20Reference) (OtherComp :type Primitive%20Component%20Object%20Reference) (OtherBodyIndex :type Integer) (bFromSweep :type Boolean) (SweepResult :type Hit%20Result%20Structure%20%28by%20ref%29))
  (Development|PrintString (Utilities|GetDisplayName OtherActor))
  (CallFunction|TurnChar))

(event Custom|Update%20Animation
  (bind _sprite (Variables|Default|GetSprite))
  ;[0.07812 0.4041 1] Handle Animation
  (if (AI|Components|NavMovement|IsFalling (Variables|Character|GetCharacterMovement))
    (Sprite|SetFlipbook _sprite "/Game/Enemies/Custom_Enemy_Assets/Mushroom-Idle1.Mushroom-Idle1")
    (else
      (Sprite|SetFlipbook _sprite (select (> (Math|Vector|VectorLength (Transformation|GetVelocity)) 0.0) "/Game/Enemies/Custom_Enemy_Assets/Mushroom-Run1.Mushroom-Run1" "/Game/Enemies/Custom_Enemy_Assets/Mushroom-Idle1.Mushroom-Idle1")))))

(event Custom|MoveToTarget
  ;[0.5776 0.5841 0.2502] Move to Target
  (bind _asbp_2dsidescroller_character (Utilities|Casting|CastToBP_2DSidescrollerCharacter (Variables|Default|GetTarget)))
  (Pawn|Input|AddMovementInput (Math|Vector|MakeVector (.x (Math|Vector|Normalize (- (Transformation|GetActorLocation _asbp_2dsidescroller_character) (Transformation|GetActorLocation)))) 0.0 0.0) (Variables|Default|GetspeedScale) false))

(event EventTick
  (params (DeltaSeconds :type Float%20%28single-precision%29))
  ;[0.3772 1 0.4017] Tick - Update Animation
  (Pawn|Input|AddMovementInput (Transformation|GetActorForwardVector) 1.0 false))

(fn ConstructionScript)

(fn TurnChar
  (Transformation|SetActorRotation (Math|Rotator|CombineRotators (Transformation|GetActorRotation) "0.000000,180.000000,0.000000")))