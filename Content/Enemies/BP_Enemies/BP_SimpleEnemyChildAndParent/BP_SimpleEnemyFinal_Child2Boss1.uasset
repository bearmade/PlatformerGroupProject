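; A 2D sidescroller boss, built as a child of the simple enemy Blueprint, that fires projectiles at the player.
; When the player enters PlayerDetection, it plays a vine puppet attack flipbook, spawns a projectile after a delay, then starts a cooldown.
; BP_Blast leaving the Box costs one health, and Tick destroys the actor at zero.
; BeginPlay removes HitDetection; UpdateAnimation selects the same flipbook in every branch.
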(event OnComponentBeginOverlap(PlayerDetection)
  (params (OverlappedComponent :type Primitive%20Component%20Object%20Reference) (OtherActor :type Actor%20Object%20Reference) (OtherComp :type Primitive%20Component%20Object%20Reference) (OtherBodyIndex :type Integer) (bFromSweep :type Boolean) (SweepResult :type Hit%20Result%20Structure%20%28by%20ref%29))
  (if (Variables|Default|GetbossCanAttack)
    (Utilities|Casting|CastToBP_2DSidescrollerCharacter OtherActor)
    (Sprite|SetFlipbook (Variables|Default|GetSprite) "/Game/Enemies/Custom_Enemy_Assets/Vine_Puppet_Sprite/Boss1_Attack/AttackOne-SheetVinePuppet1.AttackOne-SheetVinePuppet1")
    (Utilities|FlowControl|Delay 0.9)
    (Game|SpawnActorfromClass "/Game/Enemies/BP_EnemyProjectile1.BP_EnemyProjectile1_C" (Transformation|GetWorldTransform (Variables|Default|GetSpawnProjectile)) "Undefined" "MultiplyWithRoot" 0 0)
    (Sprite|SetFlipbook (Variables|Default|GetSprite) "/Game/Enemies/Custom_Enemy_Assets/Vine_Puppet_Sprite/Boss1_Idle/bossSpriteAnim-Sheet1.bossSpriteAnim-Sheet1")
    (Variables|Default|SetbossCanAttack false)
    (Utilities|FlowControl|Delay 3.0)
    (Variables|Default|SetbossCanAttack true)))

(event OnComponentEndOverlap(PlayerDetection)
  (params (OverlappedComponent :type Primitive%20Component%20Object%20Reference) (OtherActor :type Actor%20Object%20Reference) (OtherComp :type Primitive%20Component%20Object%20Reference) (OtherBodyIndex :type Integer))
  (Utilities|Casting|CastToBP_2DSidescrollerCharacter OtherActor)
  (Sprite|SetFlipbook (Variables|Default|GetSprite) "/Game/Enemies/Custom_Enemy_Assets/Vine_Puppet_Sprite/Boss1_Idle/bossSpriteAnim-Sheet1.bossSpriteAnim-Sheet1")
  (Development|PrintString "Boss Detection"))

(event OnComponentEndOverlap(Box)
  (params (OverlappedComponent :type Primitive%20Component%20Object%20Reference) (OtherActor :type Actor%20Object%20Reference) (OtherComp :type Primitive%20Component%20Object%20Reference) (OtherBodyIndex :type Integer))
  (Utilities|Casting|CastToBP_Blast OtherActor)
  (Development|PrintString "Boss1Hit")
  (Sprite|SetFlipbook (Variables|Default|GetSprite) "/Game/Enemies/Custom_Enemy_Assets/Vine_Puppet_Sprite/Boss1_Idle/bossSpriteAnim-Sheet1.bossSpriteAnim-Sheet1")
  (Variables|Default|SetBoss%20Health (- (Variables|Default|GetBoss%20Health) 1.0)))

(event Custom|UpdateAnimation
  (bind _sprite (Variables|Default|GetSprite))
  (if (AI|Components|NavMovement|IsFalling (Variables|Character|GetCharacterMovement))
    (Sprite|SetFlipbook _sprite "/Game/Enemies/Custom_Enemy_Assets/Vine_Puppet_Sprite/Boss1_Idle/bossSpriteAnim-Sheet1.bossSpriteAnim-Sheet1")
    (else
      (Sprite|SetFlipbook _sprite (select (> (Math|Vector|VectorLength (Transformation|GetVelocity)) 0.0) "/Game/Enemies/Custom_Enemy_Assets/Vine_Puppet_Sprite/Boss1_Idle/bossSpriteAnim-Sheet1.bossSpriteAnim-Sheet1" "/Game/Enemies/Custom_Enemy_Assets/Vine_Puppet_Sprite/Boss1_Idle/bossSpriteAnim-Sheet1.bossSpriteAnim-Sheet1")))))

(event EventBeginPlay
  (Components|DestroyComponent (Variables|Default|GetHit%20Detection))
  (Variables|Default|SetbossCanAttack true))

(event EventTick
  (params (DeltaSeconds :type Float%20%28single-precision%29))
  (if (<= (Variables|Default|GetBoss%20Health) 0.0)
    (Actor|DestroyActor)))

(fn ConstructionScript
  (|CallParentFunction))