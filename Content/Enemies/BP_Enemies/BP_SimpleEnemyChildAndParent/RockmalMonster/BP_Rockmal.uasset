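; Rockmal monster, a simple 2D sidescroller enemy that moves forward, turns on wall overlaps and removes its player detection at spawn.
; Attack overlaps damage and knock back the player once IsAttacking is set; the first overlap only sets that flag.
; Player weapon overlaps only flash the sprite red on exit; zero health triggers smoke, a heart drop and destruction from Tick.
; AnimationUpdate uses Kicker flipbooks, while attacks use Rockmal ones.
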(event OnComponentHit(CapsuleComponent)
  (params (HitComponent :type Primitive%20Component%20Object%20Reference) (OtherActor :type Actor%20Object%20Reference) (OtherComp :type Primitive%20Component%20Object%20Reference) (NormalImpulse :type Vector :default "0, 0, 0") (Hit :type Hit%20Result%20Structure%20%28by%20ref%29))
  (Variables|Default|SetisMovingRight? (not (Variables|Default|GetisMovingRight?))))

(event OnComponentBeginOverlap(AttackCollision)
  (params (OverlappedComponent :type Primitive%20Component%20Object%20Reference) (OtherActor :type Actor%20Object%20Reference) (OtherComp :type Primitive%20Component%20Object%20Reference) (OtherBodyIndex :type Integer) (bFromSweep :type Boolean) (SweepResult :type Hit%20Result%20Structure%20%28by%20ref%29))
  (if (Variables|Default|GetIsAttacking)
    (bind _asbp_2dsidescroller_character (Utilities|Casting|CastToBP_2DSidescrollerCharacter OtherActor))
    (Sprite|SetFlipbook (Variables|Default|GetSprite) "/Game/Enemies/Custom_Enemy_Assets/RockMal_Sprites/Rockmal_attack_long_ani1.Rockmal_attack_long_ani1")
    (Default|SubHealth _asbp_2dsidescroller_character -1)
    (Utilities|FlowControl|Delay 0.5)
    (Default|KnockBack _asbp_2dsidescroller_character)
    (else
      (Variables|Default|SetIsAttacking true))))

(event OnComponentEndOverlap(AttackCollision)
  (params (OverlappedComponent :type Primitive%20Component%20Object%20Reference) (OtherActor :type Actor%20Object%20Reference) (OtherComp :type Primitive%20Component%20Object%20Reference) (OtherBodyIndex :type Integer))
  (Utilities|Casting|CastToBP_2DSidescrollerCharacter OtherActor)
  (Utilities|FlowControl|Delay 0.2)
  (Sprite|SetFlipbook (Variables|Default|GetSprite) "/Game/Enemies/Custom_Enemy_Assets/RockMal_Sprites/Rockmal_walk_ani1.Rockmal_walk_ani1"))

(event OnComponentEndOverlap(HitDetection)
  (params (OverlappedComponent :type Primitive%20Component%20Object%20Reference) (OtherActor :type Actor%20Object%20Reference) (OtherComp :type Primitive%20Component%20Object%20Reference) (OtherBodyIndex :type Integer))
  ;[0.229 0.6146 0.1488] Enemy Hit Detection
  (Utilities|FlowControl|Sequence
    (:then_0
      (Utilities|Casting|CastToBP_Blast OtherActor))
    (:then_1
      (Utilities|Casting|CastToBP_Boomerang OtherActor))
    (:then_2
      (Utilities|Casting|CastToBP_Hatchet OtherActor))
    (:then_3
      (Utilities|Casting|CastToBP_WaterJets OtherActor))
    (:then_4
      (Utilities|Casting|CastToBP_GroundPoundBlast OtherActor)))
  (Sprite|SetSpriteColor (Variables|Default|GetSprite) "(R=1.000000,G=0.000000,B=0.000000,A=0.500000)")
  (Utilities|FlowControl|Delay 0.1)
  (Sprite|SetSpriteColor (Variables|Default|GetSprite) "(R=1.000000,G=1.000000,B=1.000000,A=1.000000)"))

(event OnComponentBeginOverlap(WallDetection)
  (params (OverlappedComponent :type Primitive%20Component%20Object%20Reference) (OtherActor :type Actor%20Object%20Reference) (OtherComp :type Primitive%20Component%20Object%20Reference) (OtherBodyIndex :type Integer) (bFromSweep :type Boolean) (SweepResult :type Hit%20Result%20Structure%20%28by%20ref%29))
  (Transformation|SetActorRotation (Math|Rotator|CombineRotators (Transformation|GetActorRotation) "0.000000,180.000000,0.000000")))

(event OnComponentBeginOverlap(PlayerDetection)
  (params (OverlappedComponent :type Primitive%20Component%20Object%20Reference) (OtherActor :type Actor%20Object%20Reference) (OtherComp :type Primitive%20Component%20Object%20Reference) (OtherBodyIndex :type Integer) (bFromSweep :type Boolean) (SweepResult :type Hit%20Result%20Structure%20%28by%20ref%29))
  (Utilities|Casting|CastToBP_2DSidescrollerCharacter OtherActor))

(event OnComponentEndOverlap(PlayerDetection)
  (params (OverlappedComponent :type Primitive%20Component%20Object%20Reference) (OtherActor :type Actor%20Object%20Reference) (OtherComp :type Primitive%20Component%20Object%20Reference) (OtherBodyIndex :type Integer))
  (Utilities|Casting|CastToBP_2DSidescrollerCharacter OtherActor))

(event Custom|MovingLeftRight
  (Pawn|Input|AddMovementInput (Math|Vector|SelectVector "1.000000,0.000000,0.000000" "-1.000000,0.000000,0.000000" (Variables|Default|GetisMovingRight?)) 1.0 false))

(event Custom|Direction
  (Transformation|SetRelativeRotation (Variables|Default|GetSprite) (Math|Rotator|MakeRotator 0.0 0.0 (Math|Float|SelectFloat 0.0 1.8e+02 (Variables|Default|GetisMovingRight?))) false false)
  (CallFunction|MovingLeftRight)
  (Utilities|FlowControl|Delay 3.0))

(event Custom|AnimationUpdate
  (Sprite|SetFlipbook (Variables|Default|GetSprite) (select (> (Math|Vector|VectorLength (Transformation|GetVelocity)) 0.0) "/Game/Enemies/Custom_Enemy_Assets/Kicker_Sprites/Kicker_Walk_Flipbook.Kicker_Walk_Flipbook" "/Game/Enemies/Custom_Enemy_Assets/Kicker_Sprites/Kicker_Idle_Flipbook.Kicker_Idle_Flipbook")))

(event EventBeginPlay
  (Components|DestroyComponent (Variables|Default|GetPlayerDetection)))

(event EventTick
  (params (DeltaSeconds :type Float%20%28single-precision%29))
  (CallFunction|MoveForward)
  (if (<= (Variables|Default|Gethealth) 0.0)
    (Sprite|SetFlipbook (Variables|Default|GetSprite) "/Game/Enemies/Custom_Enemy_Assets/Death_Sprites/DeathSmoke1.DeathSmoke1")
    (Utilities|FlowControl|Delay 0.2)
    (CallFunction|HeartDrop)
    (Actor|DestroyActor)))

(fn ConstructionScript
  (|CallParentFunction))