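; BP_FlyingEnemy is a child enemy Blueprint for a 2D sidescroller that flies toward the player character.
; MovetoTarget adds movement input along the normalized direction to the target on X and Z only, scaled by SpeedScale, keeping motion in the side-view plane.
; UpdateAnimation picks the sprite flipbook from falling state and velocity.
; When the player leaves FollowCollision, it clears Following and resets the flipbook.
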(event OnComponentEndOverlap(FollowCollision)
  (params (OverlappedComponent :type Primitive%20Component%20Object%20Reference) (OtherActor :type Actor%20Object%20Reference) (OtherComp :type Primitive%20Component%20Object%20Reference) (OtherBodyIndex :type Integer))
  (Utilities|Casting|CastToBP_2DSidescrollerCharacter OtherActor)
  (Variables|Default|SetbFollowing false)
  (Sprite|SetFlipbook (Variables|Default|GetSprite)))

(event EventBeginPlay
  (|CallParentFunction) ; This node is disabled and will not be called.\nDrag off pins to build functionality.
)

(event Collision|EventActorBeginOverlap
  (params (OtherActor :type Actor%20Object%20Reference))
  (|CallParentFunction OtherActor) ; This node is disabled and will not be called.\nDrag off pins to build functionality.
)

(event EventTick
  (params (DeltaSeconds :type Float%20%28single-precision%29))
  (|CallParentFunction DeltaSeconds) ; This node is disabled and will not be called.\nDrag off pins to build functionality.
)

(event EventUpdateAnimation
  (bind _sprite (Variables|Default|GetSprite))
  (if (AI|Components|NavMovement|IsFalling (Variables|Character|GetCharacterMovement))
    (Sprite|SetFlipbook _sprite)
    (else
      (Sprite|SetFlipbook _sprite (select (> (Math|Vector|VectorLength (Transformation|GetVelocity)) 0.0) 0 0)))))

(event EventMovetoTarget
  (bind _asbp_2dsidescroller_character (Utilities|Casting|CastToBP_2DSidescrollerCharacter (Variables|Default|GetTarget)))
  (Pawn|Input|AddMovementInput (Math|Vector|MakeVector (.x (Math|Vector|Normalize (- (Transformation|GetActorLocation _asbp_2dsidescroller_character) (Transformation|GetActorLocation)))) 0.0 (.z (Math|Vector|Normalize (- (Transformation|GetActorLocation _asbp_2dsidescroller_character) (Transformation|GetActorLocation))))) (Variables|Default|GetspeedScale) false))

(fn ConstructionScript
  (|CallParentFunction))