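; Melee enemy child Blueprint for a 2D sidescroller that damages the player and swaps sprite flipbooks for movement, falling and attacks.
; Attack starts a looping timer that checks HitBox against Target, applying damage and briefly setting IsAttacking, which pauses the parent's Tick.
; Leaving AttackCollision clears that timer with a zero-time call and resumes following, while leaving FollowCollision stops following.
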(event OnComponentEndOverlap(AttackCollision)
  (params (OverlappedComponent :type Primitive%20Component%20Object%20Reference) (OtherActor :type Actor%20Object%20Reference) (OtherComp :type Primitive%20Component%20Object%20Reference) (OtherBodyIndex :type Integer))
  (Utilities|Casting|CastToBP_2DSidescrollerCharacter OtherActor)
  (Utilities|Time|SetTimerbyEvent (delegate Custom|CheckForHit) 0.0)
  (Variables|Default|SetbFollowing true))

(event OnComponentEndOverlap(FollowCollision)
  (params (OverlappedComponent :type Primitive%20Component%20Object%20Reference) (OtherActor :type Actor%20Object%20Reference) (OtherComp :type Primitive%20Component%20Object%20Reference) (OtherBodyIndex :type Integer))
  (Utilities|Casting|CastToBP_2DSidescrollerCharacter OtherActor)
  (Variables|Default|SetbFollowing false)
  (Sprite|SetFlipbook (Variables|Default|GetSprite)))

(event Custom|CheckForHit
  (Variables|Default|SetisAttacking false)
  (if (Collision|IsOverlappingActor (Variables|Default|GetHitBox) (Variables|Default|GetTarget) :!class /Script/Engine.PrimitiveComponent)
    (Variables|Default|SetisAttacking true)
    (Sprite|SetFlipbook (Variables|Default|GetSprite))
    (Utilities|Time|SetTimerbyEvent (delegate Custom|StopAttacking) 0.2)
    (Utilities|Casting|CastToBP_2DSidescrollerCharacter (Variables|Default|GetTarget))
    (Game|Damage|ApplyDamage (Game|GetPlayerCharacter 0) 5.0 0 0)))

(event Custom|StopAttacking
  (Variables|Default|SetisAttacking false)
  (Sprite|SetFlipbook (Variables|Default|GetSprite)))

(event EventBeginPlay
  (|CallParentFunction) ; This node is disabled and will not be called.\nDrag off pins to build functionality.
)

(event Collision|EventActorBeginOverlap
  (params (OtherActor :type Actor%20Object%20Reference))
  (|CallParentFunction OtherActor) ; This node is disabled and will not be called.\nDrag off pins to build functionality.
)

(event EventTick
  (params (DeltaSeconds :type Float%20%28single-precision%29))
  (if (not (Variables|Default|GetisAttacking))
    (|CallParentFunction DeltaSeconds)))

(event EventAttack
  (CallFunction|CheckforHit)
  (Utilities|Time|SetTimerbyEvent (delegate Custom|CheckForHit) 0.5 true))

(event EventUpdateAnimation
  (bind _sprite (Variables|Default|GetSprite))
  (if (AI|Components|NavMovement|IsFalling (Variables|Character|GetCharacterMovement))
    (Sprite|SetFlipbook _sprite)
    (else
      (Sprite|SetFlipbook _sprite (select (> (Math|Vector|VectorLength (Transformation|GetVelocity)) 0.0) 0 0)))))

(fn ConstructionScript
  (|CallParentFunction))