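; Child Blueprint for a Gear Monkey side-scroller enemy that spawns a projectile whenever the player enters its PlayerDetection volume.
; BeginPlay destroys the HitDetection component, while capsule overlaps with five player attack types flash the sprite red without changing Health here.
; Tick watches Health and, at zero or below, shows death smoke before destroying the actor.
; Every non-death animation branch uses the same GearMonkey1 flipbook.
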(event OnComponentBeginOverlap(PlayerDetection)
  (params (OverlappedComponent :type Primitive%20Component%20Object%20Reference) (OtherActor :type Actor%20Object%20Reference) (OtherComp :type Primitive%20Component%20Object%20Reference) (OtherBodyIndex :type Integer) (bFromSweep :type Boolean) (SweepResult :type Hit%20Result%20Structure%20%28by%20ref%29))
  (Utilities|Casting|CastToBP_2DSidescrollerCharacter OtherActor)
  (Game|SpawnActorfromClass "/Game/Enemies/BP_EnemyProjectile.BP_EnemyProjectile_C" (Transformation|GetWorldTransform (Variables|Default|GetSpawnProjectile)) "Undefined" "MultiplyWithRoot" 0 0)
  (Sprite|SetFlipbook (Variables|Default|GetSprite) "/Game/Enemies/Custom_Enemy_Assets/GearMonkey_Sprites/GearMonkey1.GearMonkey1"))

(event OnComponentEndOverlap(PlayerDetection)
  (params (OverlappedComponent :type Primitive%20Component%20Object%20Reference) (OtherActor :type Actor%20Object%20Reference) (OtherComp :type Primitive%20Component%20Object%20Reference) (OtherBodyIndex :type Integer))
  (Utilities|Casting|CastToBP_2DSidescrollerCharacter OtherActor)
  (Sprite|SetFlipbook (Variables|Default|GetSprite) "/Game/Enemies/Custom_Enemy_Assets/GearMonkey_Sprites/GearMonkey1.GearMonkey1")
  (Development|PrintString "Monkey Detection"))

(event OnComponentBeginOverlap(CapsuleComponent)
  (params (OverlappedComponent :type Primitive%20Component%20Object%20Reference) (OtherActor :type Actor%20Object%20Reference) (OtherComp :type Primitive%20Component%20Object%20Reference) (OtherBodyIndex :type Integer) (bFromSweep :type Boolean) (SweepResult :type Hit%20Result%20Structure%20%28by%20ref%29))
  (Utilities|FlowControl|Sequence
    (:then_0
      (Utilities|Casting|CastToBP_Blast OtherActor))
    (:then_1
      (Utilities|Casting|CastToBP_Boomerang OtherActor))
    (:then_2
      (Utilities|Casting|CastToBP_Hatchet OtherActor))
    (:then_3
      (Utilities|Casting|CastToBP_WaterJets OtherActor))
    (:then_4
      (Utilities|Casting|CastToBP_GroundPoundBlast OtherActor)))
  (Sprite|SetSpriteColor (Variables|Default|GetSprite) "(R=1.000000,G=0.000000,B=0.000000,A=0.500000)")
  (Utilities|FlowControl|Delay 0.2)
  (Sprite|SetSpriteColor (Variables|Default|GetSprite) "(R=1.000000,G=1.000000,B=1.000000,A=1.000000)")
  (Development|PrintString "MonkeyHit")
  (Sprite|SetFlipbook (Variables|Default|GetSprite) "/Game/Enemies/Custom_Enemy_Assets/GearMonkey_Sprites/GearMonkey1.GearMonkey1"))

(event OnComponentEndOverlap(Box)
  (params (OverlappedComponent :type Primitive%20Component%20Object%20Reference) (OtherActor :type Actor%20Object%20Reference) (OtherComp :type Primitive%20Component%20Object%20Reference) (OtherBodyIndex :type Integer)))

(event Custom|UpdateAnimation
  (bind _sprite (Variables|Default|GetSprite))
  (if (AI|Components|NavMovement|IsFalling (Variables|Character|GetCharacterMovement))
    (Sprite|SetFlipbook _sprite "/Game/Enemies/Custom_Enemy_Assets/GearMonkey_Sprites/GearMonkey1.GearMonkey1")
    (else
      (Sprite|SetFlipbook _sprite (select (> (Math|Vector|VectorLength (Transformation|GetVelocity)) 0.0) "/Game/Enemies/Custom_Enemy_Assets/GearMonkey_Sprites/GearMonkey1.GearMonkey1" "/Game/Enemies/Custom_Enemy_Assets/GearMonkey_Sprites/GearMonkey1.GearMonkey1")))))

(event EventBeginPlay
  (Components|DestroyComponent (Variables|Default|GetHit%20Detection)))

(event Collision|EventActorBeginOverlap
  (params (OtherActor :type Actor%20Object%20Reference)))

(event EventTick
  (params (DeltaSeconds :type Float%20%28single-precision%29))
  (if (<= (Variables|Default|Gethealth) 0.0)
    (Sprite|SetSpriteColor (Variables|Default|GetSprite) "(R=1.000000,G=1.000000,B=1.000000,A=1.000000)")
    (Sprite|SetFlipbook (Variables|Default|GetSprite) "/Game/Enemies/Custom_Enemy_Assets/Death_Sprites/DeathSmoke1.DeathSmoke1")
    (Utilities|FlowControl|Delay 0.2)
    (Actor|DestroyActor)))

(fn ConstructionScript
  (|CallParentFunction))