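; Vine Puppeteer, the first-level boss of a 2D sidescroller, is a simple-enemy child that removes its HitDetection component and animates through flipbook swaps.
; Player overlap starts a looping timer that runs vine and seed attack animations, firing a projectile with the seed; leaving clears the cycle flag.
; Player weapons ending overlap with DamageBox flash the sprite red and reduce health.
; Tick watches health, plays the death flipbook and destroys the actor after a delay.
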(event OnComponentBeginOverlap(PlayerDetection)
  (params (OverlappedComponent :type Primitive%20Component%20Object%20Reference) (OtherActor :type Actor%20Object%20Reference) (OtherComp :type Primitive%20Component%20Object%20Reference) (OtherBodyIndex :type Integer) (bFromSweep :type Boolean) (SweepResult :type Hit%20Result%20Structure%20%28by%20ref%29))
  ;[1 1 1] Vine Puppeteer Attack Logic
  (Utilities|Casting|CastToBP_2DSidescrollerCharacter OtherActor)
  (Variables|Default|SetCycle true)
  (Utilities|Time|SetTimerbyEvent (delegate Custom|AttackCycle) 3.0 true))

(event OnComponentEndOverlap(PlayerDetection)
  (params (OverlappedComponent :type Primitive%20Component%20Object%20Reference) (OtherActor :type Actor%20Object%20Reference) (OtherComp :type Primitive%20Component%20Object%20Reference) (OtherBodyIndex :type Integer))
  (if (not (Variables|Default|GetboosDead))
    (Utilities|Casting|CastToBP_2DSidescrollerCharacter OtherActor)
    (Sprite|SetFlipbook (Variables|Default|GetSprite) "/Game/Enemies/Custom_Enemy_Assets/Vine_Puppet_Sprite/Boss1_Idle/bossSpriteAnim-Sheet1.bossSpriteAnim-Sheet1")
    (Development|PrintString "Boss Detection")
    (Variables|Default|SetCycle false)))

(event OnComponentEndOverlap(DamageBox)
  (params (OverlappedComponent :type Primitive%20Component%20Object%20Reference) (OtherActor :type Actor%20Object%20Reference) (OtherComp :type Primitive%20Component%20Object%20Reference) (OtherBodyIndex :type Integer))
  ;[1 1 1] Boss damagable box and Hue change on hit
  (if (not (Variables|Default|GetboosDead))
    (Utilities|FlowControl|Sequence
      (:then_0
        (Utilities|Casting|CastToBP_Blast OtherActor))
      (:then_1
        (Utilities|Casting|CastToBP_Hatchet OtherActor))
      (:then_2
        (Utilities|Casting|CastToBP_Boomerang OtherActor))
      (:then_3
        (Utilities|Casting|CastToBP_WaterJets OtherActor))
      (:then_4
        (Utilities|Casting|CastToBP_GroundPoundBlast OtherActor)))
    (Sprite|SetSpriteColor (Variables|Default|GetSprite) "(R=1.000000,G=0.000000,B=0.000000,A=0.500000)")
    (Utilities|FlowControl|Delay 0.2)
    (Sprite|SetSpriteColor (Variables|Default|GetSprite) "(R=1.000000,G=1.000000,B=1.000000,A=1.000000)")
    (Development|PrintString "Boss1Hit")
    (Variables|Default|SetBoss%20Health (- (Variables|Default|GetBoss%20Health) 2.0))))

(event Custom|UpdateAnimation
  (bind _sprite (Variables|Default|GetSprite))
  ;[1 1 1] Animation Update for Vine Puppeteer Boss  First Level
  (if (and (AI|Components|NavMovement|IsFalling (Variables|Character|GetCharacterMovement)) (not (Variables|Default|GetboosDead)))
    (Sprite|SetFlipbook _sprite "/Game/Enemies/Custom_Enemy_Assets/Vine_Puppet_Sprite/Boss1_Idle/bossSpriteAnim-Sheet1.bossSpriteAnim-Sheet1")
    (elif (not (Variables|Default|GetboosDead))
      (Sprite|SetFlipbook _sprite (select (> (Math|Vector|VectorLength (Transformation|GetVelocity)) 0.0) "/Game/Enemies/Custom_Enemy_Assets/Vine_Puppet_Sprite/Boss1_Idle/bossSpriteAnim-Sheet1.bossSpriteAnim-Sheet1" "/Game/Enemies/Custom_Enemy_Assets/Vine_Puppet_Sprite/Boss1_Idle/bossSpriteAnim-Sheet1.bossSpriteAnim-Sheet1")))))

(event Custom|AttackCycle
  ;[1 1 1] Scott's crude attack animation cycle
  (if (Variables|Default|GetCycle)
    (for _array_element (Utilities|Array|MakeArray (Variables|Default|GetVineAttack) (Variables|Default|GetSeedAttack))
      (Development|PrintString (Utilities|GetDisplayName _array_element))
      (if (== _array_element (Variables|Default|GetVineAttack))
        (Variables|Default|SetVine true)
        (Variables|Default|SetSeed false)
        (if (Variables|Default|GetVine)
          (Utilities|FlowControl|Sequence
            (:then_0
              (Utilities|FlowControl|DoOnce false :!label _label
                (:Completed
                  (Sprite|SetFlipbook (Variables|Default|GetSprite) _array_element)
                  (Variables|Default|SetVine false)
                  (Variables|Default|SetSeed true))))
            (:then_1
              (Utilities|FlowControl|Delay 2.5)
              (goto _label Reset))))
        (else
          (Variables|Default|SetVine false)
          (Variables|Default|SetSeed true)
          (if (Variables|Default|GetSeed)
            (Utilities|FlowControl|Delay 1.5)
            (Sprite|SetFlipbook (Variables|Default|GetSprite) _array_element)
            (Utilities|FlowControl|Delay 0.9)
            (Game|SpawnActorfromClass "/Game/Enemies/BP_EnemyProjectile1.BP_EnemyProjectile1_C" (Transformation|GetWorldTransform (Variables|Default|GetSpawnProjectile)) "Undefined" "MultiplyWithRoot" 0 0)
            (Variables|Default|SetVine true)
            (Variables|Default|SetSeed false)))))
    (elif (not (Variables|Default|GetboosDead))
      (Sprite|SetFlipbook (Variables|Default|GetSprite) "/Game/Enemies/Custom_Enemy_Assets/Vine_Puppet_Sprite/Boss1_Idle/bossSpriteAnim-Sheet1.bossSpriteAnim-Sheet1"))))

(event EventBeginPlay
  (Components|DestroyComponent (Variables|Default|GetHit%20Detection))
  (Variables|Default|SetbossCanAttack true))

(event EventTick
  (params (DeltaSeconds :type Float%20%28single-precision%29))
  (if (<= (Variables|Default|GetBoss%20Health) 0.0)
    (Variables|Default|SetboosDead true)
    (Variables|Default|SetCycle false)
    (Utilities|FlowControl|Delay 0.2)
    (Sprite|SetFlipbook (Variables|Default|GetSprite) "/Game/Enemies/Custom_Enemy_Assets/Vine_Puppet_Sprite/Boss1_Death/Vine_Puppet_Death.Vine_Puppet_Death")
    (Components|Timeline|SetLooping (Variables|Default|GetSprite) false)
    (Utilities|FlowControl|Delay 5.0)
    (Actor|DestroyActor)))

(fn ConstructionScript
  (|CallParentFunction))