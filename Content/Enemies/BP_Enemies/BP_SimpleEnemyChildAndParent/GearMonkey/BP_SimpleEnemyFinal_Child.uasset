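; Gear Monkey child of the simple enemy Blueprint: a ranged enemy that fires projectiles at the side-scroller player.
; Player detection overlap starts a delay-based attack loop spawning BP_EnemyProjectile until the player leaves, and BeginPlay destroys the HitDetection component.
; Capsule overlaps with player weapons only flash the sprite red and reset its flipbook, without changing Health.
; Tick watches Health, calling HeartDrop and showing smoke before destroying the actor at zero.
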(event OnComponentBeginOverlap(PlayerDetection)
  (params (OverlappedComponent :type Primitive%20Component%20Object%20Reference) (OtherActor :type Actor%20Object%20Reference) (OtherComp :type Primitive%20Component%20Object%20Reference) (OtherBodyIndex :type Integer) (bFromSweep :type Boolean) (SweepResult :type Hit%20Result%20Structure%20%28by%20ref%29))
  (Variables|Default|SetinRange true)
  (Utilities|Casting|CastToBP_2DSidescrollerCharacter OtherActor)
  (if (not (Variables|Default|GetIsAttacking))
    (Sprite|SetFlipbook (Variables|Default|GetSprite) "/Game/Enemies/Custom_Enemy_Assets/GearMonkey_Sprites/Flipbook_BrassGearMonkey_Attack.Flipbook_BrassGearMonkey_Attack" :!label _label)
    (Utilities|FlowControl|Delay 1.0)
    (Game|SpawnActorfromClass "/Game/Enemies/Enemy_Projectiles/BP_EnemyProjectile.BP_EnemyProjectile_C" (Transformation|GetWorldTransform (Variables|Default|GetSpawnProjectile)) "Undefined" "MultiplyWithRoot" 0 0)
    (Variables|Default|SetIsAttacking true)
    (Sprite|SetFlipbook (Variables|Default|GetSprite) "/Game/Enemies/Custom_Enemy_Assets/GearMonkey_Sprites/Flipbook_BrassMonkeyIdle.Flipbook_BrassMonkeyIdle")
    (Utilities|FlowControl|Delay 1.0)
    (if (Variables|Default|GetinRange)
      (goto _label))))

(event OnComponentEndOverlap(PlayerDetection)
  (params (OverlappedComponent :type Primitive%20Component%20Object%20Reference) (OtherActor :type Actor%20Object%20Reference) (OtherComp :type Primitive%20Component%20Object%20Reference) (OtherBodyIndex :type Integer))
  (Utilities|Casting|CastToBP_2DSidescrollerCharacter OtherActor)
  (Sprite|SetFlipbook (Variables|Default|GetSprite) "/Game/Enemies/Custom_Enemy_Assets/GearMonkey_Sprites/Flipbook_BrassMonkeyIdle.Flipbook_BrassMonkeyIdle")
  (Variables|Default|SetIsAttacking false)
  (Variables|Default|SetinRange false))

(event OnComponentBeginOverlap(CapsuleComponent)
  (params (OverlappedComponent :type Primitive%20Component%20Object%20Reference) (OtherActor :type Actor%20Object%20Reference) (OtherComp :type Primitive%20Component%20Object%20Reference) (OtherBodyIndex :type Integer) (bFromSweep :type Boolean) (SweepResult :type Hit%20Result%20Structure%20%28by%20ref%29))
  (Utilities|FlowControl|Sequence
    (:then_0
      (Utilities|Casting|CastToBP_Blast OtherActor))
    (:then_1
      (Utilities|Casting|CastToBP_Boomerang OtherActor))
    (:then_2
      (Utilities|Casting|CastToBP_Hatchet OtherActor))
    (:then_3
      (Utilities|Casting|CastToBP_WaterJets OtherActor))
    (:then_4
      (Utilities|Casting|CastToBP_GroundPoundBlast OtherActor)))
  (Sprite|SetSpriteColor (Variables|Default|GetSprite) "(R=1.000000,G=0.000000,B=0.000000,A=0.500000)")
  (Utilities|FlowControl|Delay 0.2)
  (Sprite|SetSpriteColor (Variables|Default|GetSprite) "(R=1.000000,G=1.000000,B=1.000000,A=1.000000)")
  (Development|PrintString "MonkeyHit")
  (Sprite|SetFlipbook (Variables|Default|GetSprite) "/Game/Enemies/Custom_Enemy_Assets/GearMonkey_Sprites/Flipbook_BrassMonkeyIdle.Flipbook_BrassMonkeyIdle"))

(event OnComponentEndOverlap(Box)
  (params (OverlappedComponent :type Primitive%20Component%20Object%20Reference) (OtherActor :type Actor%20Object%20Reference) (OtherComp :type Primitive%20Component%20Object%20Reference) (OtherBodyIndex :type Integer)))

(event Custom|UpdateAnimation
  (if (not (Variables|Default|GetIsAttacking))
    (Sprite|SetFlipbook (Variables|Default|GetSprite) "/Game/Enemies/Custom_Enemy_Assets/GearMonkey_Sprites/Flipbook_BrassMonkeyIdle.Flipbook_BrassMonkeyIdle")))

(event EventBeginPlay
  ;[1 1 1] Destroy hit detection component
  (Components|DestroyComponent (Variables|Default|GetHit%20Detection)))

(event EventTick
  (params (DeltaSeconds :type Float%20%28single-precision%29))
  (if (<= (Variables|Default|Gethealth) 0.0)
    (CallFunction|HeartDrop)
    (Sprite|SetFlipbook (Variables|Default|GetSprite) "/Game/Enemies/Custom_Enemy_Assets/Death_Sprites/DeathSmoke1.DeathSmoke1")
    (Utilities|FlowControl|Delay 0.2)
    (Actor|DestroyActor)))

(fn ConstructionScript
  (|CallParentFunction))