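; Bear trap variant of a simple 2D side-scroller enemy, apparently inheriting its components and Health from a parent Blueprint.
; Removes HitDetection at start and calls SubHealth on the player when they enter PlayerDetection.
; Tick refreshes the flipbook, which is the same sprite in every state, and destroys the actor at zero health.
; Blast overlap endings only print and reset the sprite, without changing Health here.
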(event OnComponentBeginOverlap(PlayerDetection)
  (params (OverlappedComponent :type Primitive%20Component%20Object%20Reference) (OtherActor :type Actor%20Object%20Reference) (OtherComp :type Primitive%20Component%20Object%20Reference) (OtherBodyIndex :type Integer) (bFromSweep :type Boolean) (SweepResult :type Hit%20Result%20Structure%20%28by%20ref%29))
  (bind _asbp_2dsidescroller_character (Utilities|Casting|CastToBP_2DSidescrollerCharacter OtherActor))
  (Default|SubHealth _asbp_2dsidescroller_character -1))

(event OnComponentEndOverlap(PlayerDetection)
  (params (OverlappedComponent :type Primitive%20Component%20Object%20Reference) (OtherActor :type Actor%20Object%20Reference) (OtherComp :type Primitive%20Component%20Object%20Reference) (OtherBodyIndex :type Integer))
  (Utilities|Casting|CastToBP_2DSidescrollerCharacter OtherActor)
  (Sprite|SetFlipbook (Variables|Default|GetSprite) "/Game/Enemies/Custom_Enemy_Assets/Bear_Trap_Sprites/beartrap_sprite1.beartrap_sprite1")
  (Development|PrintString "BearTrapDetection"))

(event OnComponentEndOverlap(Box)
  (params (OverlappedComponent :type Primitive%20Component%20Object%20Reference) (OtherActor :type Actor%20Object%20Reference) (OtherComp :type Primitive%20Component%20Object%20Reference) (OtherBodyIndex :type Integer))
  (Utilities|Casting|CastToBP_Blast OtherActor)
  (Development|PrintString "BearTrapHit")
  (Sprite|SetFlipbook (Variables|Default|GetSprite) "/Game/Enemies/Custom_Enemy_Assets/Bear_Trap_Sprites/beartrap_sprite1.beartrap_sprite1"))

(event Custom|UpdateAnimation
  (bind _sprite (Variables|Default|GetSprite))
  (if (AI|Components|NavMovement|IsFalling (Variables|Character|GetCharacterMovement))
    (Sprite|SetFlipbook _sprite "/Game/Enemies/Custom_Enemy_Assets/Bear_Trap_Sprites/beartrap_sprite1.beartrap_sprite1")
    (else
      (Sprite|SetFlipbook _sprite (select (> (Math|Vector|VectorLength (Transformation|GetVelocity)) 0.0) "/Game/Enemies/Custom_Enemy_Assets/Bear_Trap_Sprites/beartrap_sprite1.beartrap_sprite1" "/Game/Enemies/Custom_Enemy_Assets/Bear_Trap_Sprites/beartrap_sprite1.beartrap_sprite1")))))

(event EventBeginPlay
  (Components|DestroyComponent (Variables|Default|GetHit%20Detection)))

(event Collision|EventActorBeginOverlap
  (params (OtherActor :type Actor%20Object%20Reference)))

(event EventTick
  (params (DeltaSeconds :type Float%20%28single-precision%29))
  (CallFunction|UpdateAnimation)
  (if (<= (Variables|Default|Gethealth) 0.0)
    (Actor|DestroyActor)))

(fn ConstructionScript
  (|CallParentFunction))