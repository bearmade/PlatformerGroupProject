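; Shard spider enemy for a 2D sidescroller that knocks back and damages the player on contact with its hit volume.
; Tick bobs the sprite, launch pad and zap collision on a sine wave, sets the same jellyfish zap flipbook for every movement state, and handles death with smoke, a heart drop and destruction.
; Player weapon overlaps only flash the sprite red and restore an idle flipbook, while player detection triggers no behavior.
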(event OnComponentBeginOverlap(CapsuleComponent)
  (params (OverlappedComponent :type Primitive%20Component%20Object%20Reference) (OtherActor :type Actor%20Object%20Reference) (OtherComp :type Primitive%20Component%20Object%20Reference) (OtherBodyIndex :type Integer) (bFromSweep :type Boolean) (SweepResult :type Hit%20Result%20Structure%20%28by%20ref%29))
  (Utilities|FlowControl|Sequence
    (:then_0
      (Utilities|Casting|CastToBP_Blast OtherActor))
    (:then_1
      (Utilities|Casting|CastToBP_Boomerang OtherActor))
    (:then_2
      (Utilities|Casting|CastToBP_Hatchet OtherActor))
    (:then_3
      (Utilities|Casting|CastToBP_WaterJets OtherActor))
    (:then_4
      (Utilities|Casting|CastToBP_GroundPoundBlast OtherActor)))
  (Sprite|SetSpriteColor (Variables|Default|GetSprite) "(R=1.000000,G=0.000000,B=0.000000,A=0.500000)")
  (Utilities|FlowControl|Delay 0.1)
  (Sprite|SetSpriteColor (Variables|Default|GetSprite) "(R=1.000000,G=1.000000,B=1.000000,A=1.000000)")
  (Sprite|SetFlipbook (Variables|Default|GetSprite) "/Game/Enemies/Custom_Enemy_Assets/ShardSpiderSprites/Shardspider_Idle-Sheet1.Shardspider_Idle-Sheet1"))

(event OnComponentBeginOverlap(HitDetection)
  (params (OverlappedComponent :type Primitive%20Component%20Object%20Reference) (OtherActor :type Actor%20Object%20Reference) (OtherComp :type Primitive%20Component%20Object%20Reference) (OtherBodyIndex :type Integer) (bFromSweep :type Boolean) (SweepResult :type Hit%20Result%20Structure%20%28by%20ref%29))
  (bind _asbp_2dsidescroller_character (Utilities|Casting|CastToBP_2DSidescrollerCharacter OtherActor))
  (Default|KnockBack _asbp_2dsidescroller_character)
  (Default|SubHealth _asbp_2dsidescroller_character -1))

(event OnComponentBeginOverlap(PlayerDetection)
  (params (OverlappedComponent :type Primitive%20Component%20Object%20Reference) (OtherActor :type Actor%20Object%20Reference) (OtherComp :type Primitive%20Component%20Object%20Reference) (OtherBodyIndex :type Integer) (bFromSweep :type Boolean) (SweepResult :type Hit%20Result%20Structure%20%28by%20ref%29))
  (Utilities|Casting|CastToBP_2DSidescrollerCharacter OtherActor))

(event OnComponentEndOverlap(PlayerDetection)
  (params (OverlappedComponent :type Primitive%20Component%20Object%20Reference) (OtherActor :type Actor%20Object%20Reference) (OtherComp :type Primitive%20Component%20Object%20Reference) (OtherBodyIndex :type Integer)))

(event Custom|UpdateAnimation
  (bind _sprite (Variables|Default|GetSprite))
  (if (AI|Components|NavMovement|IsFalling (Variables|Character|GetCharacterMovement))
    (Sprite|SetFlipbook _sprite "/Game/Enemies/Custom_Enemy_Assets/JellyFish_Sprites/JellyFish_Sprites_Zap1.JellyFish_Sprites_Zap1")
    (else
      (Sprite|SetFlipbook _sprite (select (> (Math|Vector|VectorLength (Transformation|GetVelocity)) 0.0) "/Game/Enemies/Custom_Enemy_Assets/JellyFish_Sprites/JellyFish_Sprites_Zap1.JellyFish_Sprites_Zap1" "/Game/Enemies/Custom_Enemy_Assets/JellyFish_Sprites/JellyFish_Sprites_Zap1.JellyFish_Sprites_Zap1")))))

(event EventBeginPlay
  (Variables|Default|SetRelativeStartingLocation (.z (.location (Transformation|GetRelativeTransform (Variables|Default|GetSprite))))))

(event Collision|EventActorBeginOverlap
  (params (OtherActor :type Actor%20Object%20Reference)))

(event EventTick
  (params (DeltaSeconds :type Float%20%28single-precision%29))
  (Transformation|SetRelativeLocation (Variables|Default|GetSprite) (Math|Vector|MakeVector 0.0 0.0 (+ (Variables|Default|GetRelativeStartingLocation) (* (Math|Trig|Sin(Degrees) (* (Actor|GetGameTimeSinceCreation) (Variables|Default|GetBobbingSpeed))) (Variables|Default|GetBobbing%20Distance)))) false false)
  (CallFunction|UpdateAnimation)
  (if (<= (Variables|Default|Gethealth) 0.0)
    (Sprite|SetFlipbook (Variables|Default|GetSprite) "/Game/Enemies/Custom_Enemy_Assets/Death_Sprites/DeathSmoke1.DeathSmoke1")
    (Utilities|FlowControl|Delay 0.2)
    (CallFunction|HeartDrop)
    (Actor|DestroyActor)))

(fn ConstructionScript
  (|CallParentFunction))