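; Mushroom enemy for a 2D sidescroller, with patrol helpers, flipbook states and death handling.
; Wall and ledge overlaps flip its facing for forward movement, and Tick swaps to smoke and destroys it at zero health.
; Player weapon overlaps ending on HitDetection briefly show a hit flipbook without changing health; player detection only prints "attack".
; Chase logic is disconnected, and nothing here calls the MoveForward or UpdateAnimation events at runtime.
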(event OnComponentBeginOverlap(HitDetection)
  (params (OverlappedComponent :type Primitive%20Component%20Object%20Reference) (OtherActor :type Actor%20Object%20Reference) (OtherComp :type Primitive%20Component%20Object%20Reference) (OtherBodyIndex :type Integer) (bFromSweep :type Boolean) (SweepResult :type Hit%20Result%20Structure%20%28by%20ref%29))
  ;[1 1 1] Hit detection
)

(event OnComponentEndOverlap(HitDetection)
  (params (OverlappedComponent :type Primitive%20Component%20Object%20Reference) (OtherActor :type Actor%20Object%20Reference) (OtherComp :type Primitive%20Component%20Object%20Reference) (OtherBodyIndex :type Integer))
  ;[1 1 1] Hit detection
  (Utilities|FlowControl|Sequence
    (:then_0
      (Utilities|Casting|CastToBP_Blast OtherActor))
    (:then_1
      (Utilities|Casting|CastToBP_Boomerang OtherActor))
    (:then_2
      (Utilities|Casting|CastToBP_Hatchet OtherActor))
    (:then_3
      (Utilities|Casting|CastToBP_WaterJets OtherActor))
    (:then_4
      (Utilities|Casting|CastToBP_GroundPoundBlast OtherActor)))
  (Development|PrintString "Mushroom Hit")
  (Sprite|SetFlipbook (Variables|Default|GetSprite) "/Game/Enemies/Custom_Enemy_Assets/Mushroom_Sprites/Mushroom-Hit1.Mushroom-Hit1")
  (Utilities|FlowControl|Delay 0.4)
  (Sprite|SetFlipbook (Variables|Default|GetSprite) "/Game/Enemies/Custom_Enemy_Assets/Mushroom_Sprites/Mushroom-Run1.Mushroom-Run1"))

(event OnComponentBeginOverlap(WallDetection)
  (params (OverlappedComponent :type Primitive%20Component%20Object%20Reference) (OtherActor :type Actor%20Object%20Reference) (OtherComp :type Primitive%20Component%20Object%20Reference) (OtherBodyIndex :type Integer) (bFromSweep :type Boolean) (SweepResult :type Hit%20Result%20Structure%20%28by%20ref%29))
  ;[1 1 1] Wall Detection
  (Development|PrintString (Utilities|GetDisplayName OtherActor))
  (CallFunction|TurnChar))

(event OnComponentBeginOverlap(PlayerDetection)
  (params (OverlappedComponent :type Primitive%20Component%20Object%20Reference) (OtherActor :type Actor%20Object%20Reference) (OtherComp :type Primitive%20Component%20Object%20Reference) (OtherBodyIndex :type Integer) (bFromSweep :type Boolean) (SweepResult :type Hit%20Result%20Structure%20%28by%20ref%29))
  ;[1 1 1] Attack Animation
  (Utilities|Casting|CastToBP_2DSidescrollerCharacter OtherActor)
  (Development|PrintString "attack"))

(event OnComponentEndOverlap(LedgeDetection)
  (params (OverlappedComponent :type Primitive%20Component%20Object%20Reference) (OtherActor :type Actor%20Object%20Reference) (OtherComp :type Primitive%20Component%20Object%20Reference) (OtherBodyIndex :type Integer))
  ;[1 1 1] Ledge Detection
  (Development|PrintString (Utilities|GetDisplayName OtherActor))
  (CallFunction|TurnChar))

(event OnComponentEndOverlap(PlayerDetection)
  (params (OverlappedComponent :type Primitive%20Component%20Object%20Reference) (OtherActor :type Actor%20Object%20Reference) (OtherComp :type Primitive%20Component%20Object%20Reference) (OtherBodyIndex :type Integer))
  ;[1 1 1] Attack Animation
  (Utilities|Casting|CastToBP_2DSidescrollerCharacter OtherActor))

(event Custom|Update%20Animation
  (bind _sprite (Variables|Default|GetSprite))
  ;[0.07812 0.4041 1] Handle Animation
  (if (AI|Components|NavMovement|IsFalling (Variables|Character|GetCharacterMovement))
    (Sprite|SetFlipbook _sprite "/Game/Enemies/Custom_Enemy_Assets/Mushroom_Sprites/Mushroom-Idle1.Mushroom-Idle1")
    (else
      (Sprite|SetFlipbook _sprite (select (> (Math|Vector|VectorLength (Transformation|GetVelocity)) 0.0) "/Game/Enemies/Custom_Enemy_Assets/Mushroom_Sprites/Mushroom-Run1.Mushroom-Run1" "/Game/Enemies/Custom_Enemy_Assets/Mushroom_Sprites/Mushroom-Idle1.Mushroom-Idle1")))))

(event Custom|MoveToTarget
  ;[0.5776 0.5841 0.2502] Move to Target
)

(event Custom|Move%20Forward
  (Pawn|Input|AddMovementInput (Transformation|GetActorForwardVector) 1.0 false))

(event EventTick
  (params (DeltaSeconds :type Float%20%28single-precision%29))
  ;[0.3772 1 0.4017] Tick - Update Animation
  (if (<= (Variables|Default|Gethealth) 0.0)
    (Sprite|SetFlipbook (Variables|Default|GetSprite) "/Game/Enemies/Custom_Enemy_Assets/Death_Sprites/DeathSmoke1.DeathSmoke1")
    (Utilities|FlowControl|Delay 0.2)
    (Actor|DestroyActor)))

(fn ConstructionScript)

(fn TurnChar
  (Transformation|SetActorRotation (Math|Rotator|CombineRotators (Transformation|GetActorRotation) "0.000000,180.000000,0.000000")))

(fn UpdateWalkSpeed
  (params (NewWalkSpeed :type Float%20%28double-precision%29))
  (Variables|/Script/Engine.CharacterMovementComponent|SetMaxWalkSpeed (Variables|Character|GetCharacterMovement) NewWalkSpeed))