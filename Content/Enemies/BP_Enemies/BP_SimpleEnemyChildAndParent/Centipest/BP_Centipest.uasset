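; Centipest boss for the 2D sidescroller, whose defeat is scripted to lead into the game's ending.
; Player detection toggles the boss health widget and swaps level and boss music, while two ranged trigger volumes spawn acid projectiles.
; Player weapons leaving DamageBox reduce health with a red flash and impact sound.
; Tick watches for zero health, then plays death, destroys the actor, and chains delayed dialogue, ship spawn and credits after that destroy call.
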(event OnComponentBeginOverlap(PlayerDetection)
  (params (OverlappedComponent :type Primitive%20Component%20Object%20Reference) (OtherActor :type Actor%20Object%20Reference) (OtherComp :type Primitive%20Component%20Object%20Reference) (OtherBodyIndex :type Integer) (bFromSweep :type Boolean) (SweepResult :type Hit%20Result%20Structure%20%28by%20ref%29))
  ;[1 1 1] Centipest Attack Logic
  (Utilities|FlowControl|Sequence
    (:then_0
      (Utilities|Casting|CastToBP_2DSidescrollerCharacter OtherActor)
      (Utilities|FlowControl|Sequence
        (:then_0
          (Utilities|FlowControl|DoOnce false :!label _label
            (:Completed
              (bind _returnvalue (UserInterface|CreateWidget "/Game/UI/WBP_Centipide_Boss_Health.WBP_Centipide_Boss_Health_C"))
              (bind _output_get (Variables|Default|SetBossUI _returnvalue))
              (UserInterface|Viewport|AddtoViewport _output_get 0))))
        (:then_1
          (Utilities|FlowControl|Delay 1.5)
          (goto _label Reset))))
    (:then_1
      ;[1 1 1] Music Switch (Inside the boss BP for credit sequence
      (bind _asbp_2dsidescroller_character (Utilities|Casting|CastToBP_2DSidescrollerCharacter OtherActor))
      (Utilities|FlowControl|DoOnce false
        (:Completed
          (Utilities|FlowControl|Sequence
            (:then_0
              (Components|Activation|ToggleActive (stale OnComponentEndOverlap(PlayerDetection) _returnvalue))
              (bind _returnvalue_2 (Audio|SpawnSound2D "/Game/SFX/Music/2359BossTheme.2359BossTheme" 1.0 1.0 0.0 0))
              (Utilities|FlowControl|DoOnce false) ; enters at Reset
            )
            (:then_1
              (Utilities|FlowControl|DoOnce false
                (:Completed
                  (Default|StopMusic _asbp_2dsidescroller_character))))))))))

(event OnComponentEndOverlap(PlayerDetection)
  (params (OverlappedComponent :type Primitive%20Component%20Object%20Reference) (OtherActor :type Actor%20Object%20Reference) (OtherComp :type Primitive%20Component%20Object%20Reference) (OtherBodyIndex :type Integer))
  (Utilities|FlowControl|Sequence
    (:then_0
      (if (not (Variables|Default|GetboosDead))
        (Utilities|Casting|CastToBP_2DSidescrollerCharacter OtherActor)
        (Sprite|SetFlipbook (Variables|Default|GetSprite) "/Game/Enemies/Custom_Enemy_Assets/Centipest/Centipest_Idle.Centipest_Idle")
        (Development|PrintString "Boss Detection")
        (Variables|Default|SetCycle false)
        (Utilities|FlowControl|Delay 1.0)
        (Widget|RemovefromParent (Variables|Default|GetBossUI))))
    (:then_1
      ;[1 1 1] Music Switch (Inside the boss BP for credit sequence
      (Utilities|Casting|CastToBP_2DSidescrollerCharacter OtherActor)
      (Utilities|FlowControl|DoOnce false
        (:Completed
          (Components|Activation|ToggleActive (stale OnComponentBeginOverlap(PlayerDetection) _returnvalue_2))
          (bind _returnvalue (Audio|SpawnSound2D "/Game/SFX/Music/2359LevelTheme.2359LevelTheme" 1.0 1.0 0.0 0))
          (Utilities|FlowControl|DoOnce false) ; enters at Reset
        )))))

(event OnComponentBeginOverlap(RangedAttack)
  (params (OverlappedComponent :type Primitive%20Component%20Object%20Reference) (OtherActor :type Actor%20Object%20Reference) (OtherComp :type Primitive%20Component%20Object%20Reference) (OtherBodyIndex :type Integer) (bFromSweep :type Boolean) (SweepResult :type Hit%20Result%20Structure%20%28by%20ref%29))
  (Utilities|Casting|CastToBP_2DSidescrollerCharacter OtherActor)
  (Game|SpawnActorfromClass "/Game/Enemies/BP_Enemies/BP_SimpleEnemyChildAndParent/Centipest/BP_Acid.BP_Acid_C" (Transformation|GetWorldTransform (Variables|Default|GetSpawnProjectile)) "Undefined" "MultiplyWithRoot" 0 0))

(event OnComponentBeginOverlap(RangedAttack1)
  (params (OverlappedComponent :type Primitive%20Component%20Object%20Reference) (OtherActor :type Actor%20Object%20Reference) (OtherComp :type Primitive%20Component%20Object%20Reference) (OtherBodyIndex :type Integer) (bFromSweep :type Boolean) (SweepResult :type Hit%20Result%20Structure%20%28by%20ref%29))
  (Utilities|Casting|CastToBP_2DSidescrollerCharacter OtherActor)
  (Game|SpawnActorfromClass "/Game/Enemies/BP_Enemies/BP_SimpleEnemyChildAndParent/Centipest/BP_Acid1.BP_Acid1_C" (Transformation|GetWorldTransform (Variables|Default|GetSpawnProjectile)) "Undefined" "MultiplyWithRoot" 0 0))

(event OnComponentEndOverlap(DamageBox)
  (params (OverlappedComponent :type Primitive%20Component%20Object%20Reference) (OtherActor :type Actor%20Object%20Reference) (OtherComp :type Primitive%20Component%20Object%20Reference) (OtherBodyIndex :type Integer))
  ;[1 1 1] Boss damagable box and Hue change on hit
  (if true
    (Utilities|FlowControl|Sequence
      (:then_0
        (Utilities|Casting|CastToBP_Blast OtherActor))
      (:then_1
        (Utilities|Casting|CastToBP_Hatchet OtherActor))
      (:then_2
        (Utilities|Casting|CastToBP_Boomerang OtherActor))
      (:then_3
        (Utilities|Casting|CastToBP_WaterJets OtherActor))
      (:then_4
        (Utilities|Casting|CastToBP_GroundPoundBlast OtherActor)))
    (Sprite|SetSpriteColor (Variables|Default|GetSprite) "(R=1.000000,G=0.000000,B=0.000000,A=0.500000)")
    (Audio|PlaySoundatLocation "/Game/SFX/Toxic_Impact.Toxic_Impact" (Transformation|GetActorLocation) "0, 0, 0" 1.0 1.0 0.0 0 0 0 0)
    (Utilities|FlowControl|Delay 0.2)
    (Sprite|SetSpriteColor (Variables|Default|GetSprite) "(R=1.000000,G=1.000000,B=1.000000,A=1.000000)")
    (Development|PrintString "Boss1Hit")
    (Variables|Default|SetBoss%20Health (- (Variables|Default|GetBoss%20Health) 3e+01))))

(event Custom|UpdateAnimation
  (bind _sprite (Variables|Default|GetSprite))
  ;[1 1 1] Animation Update for Vine Puppeteer Boss  First Level
  (if (and (AI|Components|NavMovement|IsFalling (Variables|Character|GetCharacterMovement)) (not (Variables|Default|GetboosDead)))
    (Sprite|SetFlipbook _sprite "/Game/Enemies/Custom_Enemy_Assets/Vine_Puppet_Sprite/Boss1_Idle/bossSpriteAnim-Sheet1.bossSpriteAnim-Sheet1")
    (elif (not (Variables|Default|GetboosDead))
      (Sprite|SetFlipbook _sprite (select (> (Math|Vector|VectorLength (Transformation|GetVelocity)) 0.0) "/Game/Enemies/Custom_Enemy_Assets/Vine_Puppet_Sprite/Boss1_Idle/bossSpriteAnim-Sheet1.bossSpriteAnim-Sheet1" "/Game/Enemies/Custom_Enemy_Assets/Vine_Puppet_Sprite/Boss1_Idle/bossSpriteAnim-Sheet1.bossSpriteAnim-Sheet1")))))

(event Custom|spawn%20ship
  (if (Variables|Default|GetboosDead)
    (Utilities|FlowControl|DoOnce false
      (:Completed
        (bind _asbp_2dsidescroller_character (Utilities|Casting|CastToBP_2DSidescrollerCharacter (Game|GetPlayerCharacter 0)))
        (Input|DisableInput _asbp_2dsidescroller_character (Game|GetPlayerController 0))
        (Utilities|FlowControl|Delay 5.0)
        (Game|SpawnActorfromClass "/Game/Other/ship/Ship3.Ship3_C" (Transformation|GetWorldTransform (Variables|/Game/Player/BP_2DSidescrollerCharacter.BP_2DSidescrollerCharacter_C|Getship%20spawn _asbp_2dsidescroller_character)) "Undefined" "MultiplyWithRoot" 0 0)))))

(event EventBeginPlay
  (Components|DestroyComponent (Variables|Default|GetHit%20Detection)))

(event EventTick
  (params (DeltaSeconds :type Float%20%28single-precision%29))
  (if (<= (Variables|Default|GetBoss%20Health) 0.0)
    (Widget|RemovefromParent (Variables|Default|GetBossUI))
    (Utilities|FlowControl|Delay 0.2)
    (Utilities|FlowControl|DoOnce false
      (:Completed
        (Sprite|SetFlipbook (Variables|Default|GetSprite) "/Game/Enemies/BP_Enemies/BP_SimpleEnemyChildAndParent/Centipest/Centipest_Front_Head_Dying_Breaking-Sheet1.Centipest_Front_Head_Dying_Breaking-Sheet1")
        (Sprite|SetSpriteColor (Variables|Default|GetSprite1) "(R=0.104167,G=0.104167,B=0.104167,A=1.000000)")
        (Utilities|FlowControl|Delay 0.8)
        (Actor|DestroyActor)
        (Utilities|FlowControl|DoOnce false
          (:Completed
            (bind _returnvalue (UserInterface|CreateWidget "/Game/UI/WBP_ToxicDeathDialogue.WBP_ToxicDeathDialogue_C"))
            (UserInterface|Viewport|AddtoViewport _returnvalue 0)
            (Utilities|FlowControl|Delay 8.0)
            (CallFunction|SpawnShip)
            ;[1 1 1] End Credits
            (Utilities|FlowControl|Delay 5.0)
            (bind _foundwidgets (Widget|GetAllWidgetsOfClass "/Game/UI/WBP_WidgetHUD.WBP_WidgetHUD_C" true))
            (for _array_element _foundwidgets
              (Widget|RemovefromParent _array_element)
              (bind _returnvalue_2 (UserInterface|CreateWidget "/Game/UI/WBP_Credits.WBP_Credits_C"))
              (UserInterface|Viewport|AddtoViewport _returnvalue_2 0)
              (Audio|SpawnSound2D "/Game/SFX/Music/2359TitleTheme.2359TitleTheme" 1.0 1.0 0.0 0))))))))

(fn ConstructionScript
  (|CallParentFunction))