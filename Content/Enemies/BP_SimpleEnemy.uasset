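; BP_SimpleEnemy is a 2D side-scroller enemy that chases the player character along the X axis.
; Overlapping FollowCollision sets the target and starts following; leaving it stops the chase and restores the idle flipbook.
; While following, Tick applies movement input, picks run or idle flipbooks, and yaws the actor to face travel.
; Entering AttackCollision halts following and calls Attack, which only prints a debug string.
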(event OnComponentBeginOverlap(FollowCollision)
  (params (OverlappedComponent :type Primitive%20Component%20Object%20Reference) (OtherActor :type Actor%20Object%20Reference) (OtherComp :type Primitive%20Component%20Object%20Reference) (OtherBodyIndex :type Integer) (bFromSweep :type Boolean) (SweepResult :type Hit%20Result%20Structure%20%28by%20ref%29))
  ;[1 1 1] setFollowing
  (bind _asbp_2dsidescroller_character (Utilities|Casting|CastToBP_2DSidescrollerCharacter OtherActor))
  (Variables|Default|SetbFollowing true)
  (Variables|Default|SetTarget _asbp_2dsidescroller_character))

(event OnComponentEndOverlap(FollowCollision)
  (params (OverlappedComponent :type Primitive%20Component%20Object%20Reference) (OtherActor :type Actor%20Object%20Reference) (OtherComp :type Primitive%20Component%20Object%20Reference) (OtherBodyIndex :type Integer))
  ;[1 1 1] setFollowing
  (Utilities|Casting|CastToBP_2DSidescrollerCharacter OtherActor)
  (Variables|Default|SetbFollowing false)
  (Sprite|SetFlipbook (Variables|Default|GetSprite) "/Game/Enemies/Enemy_Idle_Flipbook.Enemy_Idle_Flipbook"))

(event OnComponentBeginOverlap(AttackCollision)
  (params (OverlappedComponent :type Primitive%20Component%20Object%20Reference) (OtherActor :type Actor%20Object%20Reference) (OtherComp :type Primitive%20Component%20Object%20Reference) (OtherBodyIndex :type Integer) (bFromSweep :type Boolean) (SweepResult :type Hit%20Result%20Structure%20%28by%20ref%29))
  (bind _target (Variables|Default|GetTarget))
  (if (== OtherActor _target)
    (Utilities|Casting|CastToBP_2DSidescrollerCharacter _target)
    (CallFunction|Attack)
    (Variables|Default|SetbFollowing false)))

(event OnComponentEndOverlap(AttackCollision)
  (params (OverlappedComponent :type Primitive%20Component%20Object%20Reference) (OtherActor :type Actor%20Object%20Reference) (OtherComp :type Primitive%20Component%20Object%20Reference) (OtherBodyIndex :type Integer)))

(event Custom|Update%20Animation
  (bind _sprite (Variables|Default|GetSprite))
  ;[1 1 1] Handle Animation
  (if (AI|Components|NavMovement|IsFalling (Variables|Character|GetCharacterMovement))
    (Sprite|SetFlipbook _sprite "/Game/Enemies/Enemy_Run_Flipbook.Enemy_Run_Flipbook")
    (else
      (Sprite|SetFlipbook _sprite (select (> (Math|Vector|VectorLength (Transformation|GetVelocity)) 0.0) "/Game/Enemies/Enemy_Run_Flipbook.Enemy_Run_Flipbook" "/Game/Enemies/Enemy_Idle_Flipbook.Enemy_Idle_Flipbook")))))

(event Custom|MoveToTarget
  ;[1 1 1] MoveToTarget
  (bind _asbp_2dsidescroller_character (Utilities|Casting|CastToBP_2DSidescrollerCharacter (Variables|Default|GetTarget)))
  (Pawn|Input|AddMovementInput (Math|Vector|MakeVector (.x (Math|Vector|Normalize (- (Transformation|GetActorLocation _asbp_2dsidescroller_character) (Transformation|GetActorLocation)))) 0.0 0.0) (Variables|Default|GetspeedScale) false))

(event Custom|Attack
  ;[1 1 1] attack
  (Development|PrintString "attack"))

(event EventBeginPlay)

(event Collision|EventActorBeginOverlap
  (params (OtherActor :type Actor%20Object%20Reference)))

(event EventTick
  (params (DeltaSeconds :type Float%20%28single-precision%29))
  ;[1 1 1] Tick - Update Animation
  (if (Variables|Default|GetbFollowing)
    (CallFunction|MovetoTarget)
    (CallFunction|UpdateAnimation)
    (Math|Float|CompareFloat (.X (Class|KismetMathLibrary|BreakVector3f (Transformation|GetVelocity))) 0.0
      (:>
        (Transformation|SetActorRotation (Math|Rotator|MakeRotator 0.0 0.0 0.0)))
      (:<
        (Transformation|SetActorRotation (Math|Rotator|MakeRotator 0.0 0.0 1.8e+02))))))

(fn ConstructionScript)