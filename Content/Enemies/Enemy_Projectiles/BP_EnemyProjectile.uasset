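; Enemy projectile actor that damages the 2D sidescroller player character on overlap.
; On hit it subtracts a fixed amount from the character's Health, destroys itself and triggers the character's KnockBack.
; If it hits nothing, it destroys itself after a short delay from BeginPlay.
; Flinging sound nodes exist but are unconnected, so no sound plays.
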(event EventBeginPlay
  (Utilities|FlowControl|Delay 1.0)
  (Actor|DestroyActor))

(event Collision|EventActorBeginOverlap
  (params (OtherActor :type Actor%20Object%20Reference))
  (bind _asbp_2dsidescroller_character (Utilities|Casting|CastToBP_2DSidescrollerCharacter OtherActor))
  (Variables|/Game/Player/BP_2DSidescrollerCharacter.BP_2DSidescrollerCharacter_C|SetHealth _asbp_2dsidescroller_character (- (Variables|/Game/Player/BP_2DSidescrollerCharacter.BP_2DSidescrollerCharacter_C|GetHealth _asbp_2dsidescroller_character) 0.5))
  (Actor|DestroyActor)
  (Default|KnockBack _asbp_2dsidescroller_character))

(event EventTick
  (params (DeltaSeconds :type Float%20%28single-precision%29)))

(fn ConstructionScript)