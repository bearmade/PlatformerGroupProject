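; BP_BoomerangPickup is a pickup that grants the boomerang to the 2D sidescroller character.
; On overlap it casts to BP_2DSidescrollerCharacter, sets HasBoomerang and destroys itself.
; From BeginPlay a looping delay chain briefly swaps its flipbook from Coin_Single to the Coin animation at random intervals, reusing coin art for the visual.
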(event EventBeginPlay
  (Utilities|FlowControl|Delay (Math|Random|RandomFloatinRange 2.0 6.0) :!label _label)
  (Sprite|SetFlipbook (Variables|Default|GetRenderComponent) "/Game/Pickups/Coin_Flipbook.Coin_Flipbook")
  (Utilities|FlowControl|Delay 0.5)
  (Sprite|SetFlipbook (Variables|Default|GetRenderComponent) "/Game/Pickups/Coin_Single_Flipbook.Coin_Single_Flipbook")
  (goto _label))

(event EventTick
  (params (DeltaSeconds :type Float%20%28single-precision%29)))

(event Collision|EventActorBeginOverlap
  (params (OtherActor :type Actor%20Object%20Reference))
  (bind _asbp_2dsidescroller_character (Utilities|Casting|CastToBP_2DSidescrollerCharacter OtherActor))
  (Variables|/Game/Player/BP_2DSidescrollerCharacter.BP_2DSidescrollerCharacter_C|SethasBoomerang _asbp_2dsidescroller_character true)
  (Actor|DestroyActor))

(fn ConstructionScript)