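; Procedural 2D level generator that spawns tile-based rooms on the XZ plane at BeginPlay.
; BeginPlay clears MapGrid, then RandomWalk steps along X or Y per the Horizontal flag, spawning a random Buildings entry at each sprite-sized cell.
; An older pipeline, disconnected from execution, builds border blocks, ledges, platforms and hazards, then runs Game of Life cellular automata to scatter coins and rare hearts.
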(event Custom|createBox
  (bind _mapwidth (Variables|Default|GetmapWidth))
  (bind _spritesize (Variables|Default|GetspriteSize))
  (bind _block (Variables|Default|Getblock))
  ;[1 1 1] draw box
  (for (_ _array_index) (Variables|Default|GetmapGrid)
    (Variables|Default|Setx (Math|Integer|%(Integer) _array_index _mapwidth))
    (Variables|Default|Sety (/ _array_index _mapwidth))
    (if (Math|Boolean|ORBoolean (== (+ (Math|Integer|%(Integer) _array_index _mapwidth) 1) (Variables|Default|GetmapHeight)) (== (+ (/ _array_index _mapwidth) 1) (Variables|Default|GetmapWidth)) (== (/ _array_index _mapwidth) 0) (== (Math|Integer|%(Integer) _array_index _mapwidth) 0))
      (bind _output_get (Variables|Default|SetvectorCoordinates (Math|Vector|MakeVector (Math|Conversions|ToFloat(Integer) (* (Variables|Default|Getx) _spritesize)) 0.0 (Math|Conversions|ToFloat(Integer) (* (Variables|Default|Gety) _spritesize)))))
      (Game|SpawnActorfromClass (Utilities|GetClass _block) (Math|Transform|MakeTransform _output_get) "Undefined" "MultiplyWithRoot" 0 0)
      (AddComponent|AddPaperTileMapComponent _block false (Math|Transform|MakeTransform _output_get)))))

(event Custom|initGrid2
  (bind _output_get (Variables|Default|SetmapSize (* (Variables|Default|GetmapHeight) (Variables|Default|GetmapWidth))))
  (for _index (range 0 _output_get)
    (Utilities|Array|SetArrayElem (Variables|Default|GetmapGrid) _index 0 true)))

(event Custom|RandomWalk
  (Variables|Default|Setx 0)
  (Variables|Default|Sety 0)
  (CallFunction|DrawRoom)
  (for _index (range 0 (Variables|Default|GetnumOfSteps))
    (if (Variables|Default|Gethorizontal)
      (Math|Integer|IncrementInt (Variables|Default|Getx)
        (:%20%20
          (CallFunction|DrawRoom)))
      (else
        (Math|Integer|IncrementInt (Variables|Default|Gety)
          (:%20%20
            (CallFunction|DrawRoom)))))))

(event Custom|DrawRoom
  (bind _spritesize (Variables|Default|GetspriteSize))
  (bind _buildings (Variables|Default|GetBuildings))
  (bind _outitem (Utilities|Array|Random _buildings))
  (bind _output_get (Variables|Default|SetvectorCoordinates (Math|Vector|MakeVector (Math|Conversions|ToFloat(Integer) (* (Variables|Default|Getx) _spritesize)) 0.0 (Math|Conversions|ToFloat(Integer) (* (Variables|Default|Gety) _spritesize)))))
  (Game|SpawnActorfromClass (Utilities|GetClass _outitem) (Math|Transform|MakeTransform _output_get) "Undefined" "MultiplyWithRoot" 0 0)
  (AddComponent|AddPaperTileMapComponent _outitem false (Math|Transform|MakeTransform _output_get)))

(event Custom|CellularAuto
  (bind _mapwidth (Variables|Default|GetmapWidth))
  (bind _tempgrid (Variables|Default|GettempGrid))
  ;[1 1 1] cellular automata
  (CallFunction|CopyArray)
  (for (_array_element _array_index) (Variables|Default|GetmapGrid)
    (Variables|Default|Setx (Math|Integer|%(Integer) _array_index _mapwidth))
    (Variables|Default|Sety (/ _array_index _mapwidth))
    (CallFunction|CountNeighbors)
    (if (and (Math|Conversions|ToBoolean(Integer) _array_element) (or (== (Variables|Default|Getneighbors) 2) (== (Variables|Default|Getneighbors) 3)))
      (Utilities|Array|SetArrayElem _tempgrid _array_index 1 true :!label _label)
      (elif (not (Math|Conversions|ToBoolean(Integer) _array_element))
        (if (== (Variables|Default|Getneighbors) 3)
          (goto _label)
          (else
            (Utilities|Array|SetArrayElem _tempgrid _array_index 0 true)))))))

(event Custom|countNeighbors
  ;[1 1 1] count neighbors
  (bind _output_get (Variables|Default|Setneighbors (+ (Utilities|Array|Get(acopy) (Variables|Default|GetmapGrid) (+ (+ (Variables|Default|Gety) 1) (* (+ (Variables|Default|Getx) 1) (Variables|Default|GetmapWidth)))) (Utilities|Array|Get(acopy) (Variables|Default|GetmapGrid) (+ (+ (Variables|Default|Gety) 0) (* (+ (Variables|Default|Getx) 1) (Variables|Default|GetmapWidth)))) (Utilities|Array|Get(acopy) (Variables|Default|GetmapGrid) (+ (+ (Variables|Default|Gety) 1) (* (+ (Variables|Default|Getx) 0) (Variables|Default|GetmapWidth)))) (Utilities|Array|Get(acopy) (Variables|Default|GetmapGrid) (+ (+ (Variables|Default|Gety) 0) (* (+ (Variables|Default|Getx) -1) (Variables|Default|GetmapWidth)))) (Utilities|Array|Get(acopy) (Variables|Default|GetmapGrid) (+ (+ (Variables|Default|Gety) -1) (* (+ (Variables|Default|Getx) 0) (Variables|Default|GetmapWidth)))) (Utilities|Array|Get(acopy) (Variables|Default|GetmapGrid) (+ (+ (Variables|Default|Gety) -1) (* (+ (Variables|Default|Getx) -1) (Variables|Default|GetmapWidth)))) (Utilities|Array|Get(acopy) (Variables|Default|GetmapGrid) (+ (+ (Variables|Default|Gety) 1) (* (+ (Variables|Default|Getx) -1) (Variables|Default|GetmapWidth)))) (Utilities|Array|Get(acopy) (Variables|Default|GetmapGrid) (+ (+ (Variables|Default|Gety) -1) (* (+ (Variables|Default|Getx) 1) (Variables|Default|GetmapWidth)))))))
  (Development|PrintString (Utilities|String|ToString(Integer) _output_get)))

(event Custom|copyArray
  ;[1 1 1] copy array
  (for (_array_element _array_index) (Variables|Default|GettempGrid)
    (Utilities|Array|SetArrayElem (Variables|Default|GetmapGrid) _array_index _array_element true)))

(event Custom|SpikeBlocks
  (bind _mapwidth (Variables|Default|GetmapWidth))
  (bind _spritesize (Variables|Default|GetspriteSize))
  ;[1 1 1] hazards
  (for (_ _array_index) (Variables|Default|GetmapGrid)
    (bind _output_get (Variables|Default|Setx (Math|Integer|%(Integer) _array_index _mapwidth)))
    (bind _output_get_2 (Variables|Default|Sety (/ _array_index _mapwidth)))
    (if (Math|Boolean|ANDBoolean (!= _output_get 0) (!= _output_get (Variables|Default|GetmapWidth)) (!= _output_get 1) (> (Math|Random|RandomIntegerinRange 0 100) 75) (Math|Boolean|ORBoolean (== _output_get_2 0) (== _output_get_2 (/ (Variables|Default|GetmapHeight) 2)) (== _output_get_2 (/ (Variables|Default|GetmapHeight) 4))) (!= _output_get 4) (!= _output_get 5) (!= _output_get 6) (!= _output_get 7) (!= _output_get (+ (Variables|Default|GetmapWidth) -1)))
      (bind _output_get_3 (Variables|Default|SetvectorCoordinates (Math|Vector|MakeVector (Math|Conversions|ToFloat(Integer) (* (Variables|Default|Getx) _spritesize)) 1e+01 (Math|Conversions|ToFloat(Integer) (* (Variables|Default|Gety) _spritesize)))))
      (Game|SpawnActorfromClass (Utilities|GetClass (.OutItem (Utilities|Array|Random (Variables|Default|Gethazards)))) (Math|Transform|MakeTransform _output_get_3) "Undefined" "MultiplyWithRoot" 0 0))))

(event Custom|drawMap
  (bind _mapheight (Variables|Default|GetmapHeight))
  (bind _spritesize (Variables|Default|GetspriteSize))
  (bind _mapwidth (Variables|Default|GetmapWidth))
  (bind _mapwidth_2 (Variables|Default|GetmapWidth))
  ;[1 1 1] draw map
  (for (_array_element _array_index) (Variables|Default|GetmapGrid)
    (Variables|Default|Setx (Math|Integer|%(Integer) _array_index _mapwidth))
    (Variables|Default|Sety (/ _array_index _mapwidth))
    (if (not (Math|Boolean|ORBoolean (== (+ (Math|Integer|%(Integer) _array_index _mapwidth) 1) (Variables|Default|GetmapHeight)) (== (+ (/ _array_index _mapwidth) 1) (Variables|Default|GetmapWidth)) (== (Math|Integer|%(Integer) _array_index _mapwidth) 0) (== (/ _array_index _mapwidth) 0) (Math|Conversions|ToBoolean(Integer) _array_element) (== (+ (Math|Integer|%(Integer) _array_index _mapwidth) 1) (/ _mapheight 2)) (== (+ (/ _array_index _mapwidth) 1) (/ _mapwidth_2 2)) (== (/ _mapheight 4) (+ (Math|Integer|%(Integer) _array_index _mapwidth) 1)) (== (/ _mapwidth_2 4) (+ (/ _array_index _mapwidth) 1))))
      (bind _output_get (Variables|Default|SetvectorCoordinates (Math|Vector|MakeVector (Math|Conversions|ToFloat(Integer) (* (Variables|Default|Getx) _spritesize)) 0.0 (Math|Conversions|ToFloat(Integer) (* (Variables|Default|Gety) _spritesize)))))
      (if (> (Math|Random|RandomInteger 100) 98)
        (Game|SpawnActorfromClass (Utilities|GetClass (Variables|Default|Getheart)) (Math|Transform|MakeTransform _output_get) "Undefined" "MultiplyWithRoot" 0 0)
        (else
          (Game|SpawnActorfromClass (Utilities|GetClass (Variables|Default|Getcoin)) (Math|Transform|MakeTransform _output_get) "Undefined" "MultiplyWithRoot" 0 0))))))

(event Custom|makePlatforms
  (bind _mapwidth (Variables|Default|GetmapWidth))
  (bind _spritesize (Variables|Default|GetspriteSize))
  (for (_ _array_index) (Variables|Default|GetmapGrid)
    (Variables|Default|Setx (Math|Integer|%(Integer) _array_index _mapwidth))
    (bind _output_get (Variables|Default|Sety (/ _array_index _mapwidth)))
    (if (and (== _output_get (- (Variables|Default|GetmapHeight) (/ (Variables|Default|GetmapHeight) 4))) (> (Math|Random|RandomIntegerinRange 0 100) 75))
      (bind _output_get_2 (Variables|Default|SetvectorCoordinates (Math|Vector|MakeVector (Math|Conversions|ToFloat(Integer) (* (Variables|Default|Getx) _spritesize)) 1e+01 (Math|Conversions|ToFloat(Integer) (* (Variables|Default|Gety) _spritesize)))))
      (Game|SpawnActorfromClass (Utilities|GetClass (.OutItem (Utilities|Array|Random (Variables|Default|Getplatforms)))) (Math|Transform|MakeTransform _output_get_2) "Undefined" "MultiplyWithRoot" 0 0))))

(event Custom|makeLedges
  (bind _mapwidth (Variables|Default|GetmapWidth))
  (bind _mapheight (Variables|Default|GetmapHeight))
  (bind _spritesize (Variables|Default|GetspriteSize))
  (bind _block (Variables|Default|Getblock))
  (bind _mapwidth_2 (Variables|Default|GetmapWidth))
  ;[1 1 1] make ledges
  (for (_ _array_index) (Variables|Default|GetmapGrid)
    (Variables|Default|Setx (Math|Integer|%(Integer) _array_index _mapwidth_2))
    (Variables|Default|Sety (/ _array_index _mapwidth_2))
    (if (and (Math|Boolean|ORBoolean (== (+ (Math|Integer|%(Integer) _array_index _mapwidth_2) 1) (/ _mapheight 2)) (== (+ (/ _array_index _mapwidth_2) 1) (/ _mapwidth 2)) (== (/ _mapheight 4) (+ (Math|Integer|%(Integer) _array_index _mapwidth_2) 1)) (== (/ _mapwidth 4) (+ (/ _array_index _mapwidth_2) 1))) (Math|Random|RandomBool))
      (bind _output_get (Variables|Default|SetvectorCoordinates (Math|Vector|MakeVector (Math|Conversions|ToFloat(Integer) (* (Variables|Default|Getx) _spritesize)) 0.0 (Math|Conversions|ToFloat(Integer) (* (Variables|Default|Gety) _spritesize)))))
      (Game|SpawnActorfromClass (Utilities|GetClass _block) (Math|Transform|MakeTransform _output_get) "Undefined" "MultiplyWithRoot" 0 0)
      (AddComponent|AddPaperTileMapComponent _block false (Math|Transform|MakeTransform _output_get)))))

(event Custom|initGrid
  ;[1 1 1] InitGrid
  (bind _output_get (Variables|Default|SetmapSize (* (Variables|Default|GetmapHeight) (Variables|Default|GetmapWidth))))
  (for _index (range 0 _output_get)
    (Utilities|Array|SetArrayElem (Variables|Default|GetmapGrid) _index (Math|Conversions|ToInteger(Boolean) (Math|Random|RandomBool)) true)))

(event EventBeginPlay
  (switch int 0
    (:0
      (CallFunction|InitGrid2)
      (CallFunction|RandomWalk))))

(event Collision|EventActorBeginOverlap
  (params (OtherActor :type Actor%20Object%20Reference)))

(event EventTick
  (params (DeltaSeconds :type Float%20%28single-precision%29)))

(fn ConstructionScript)