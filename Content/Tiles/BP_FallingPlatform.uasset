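; Falling platform actor for a 2D side-scroller that moves when the player character overlaps it, then destroys itself.
; The start location is cached on BeginPlay, and a timeline vector track offsets the platform from it without sweeping.
; Each timeline update re-arms a short destroy timer, so the platform is removed shortly after the updates stop.
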(event Custom|destroyPlatform
  (Actor|DestroyActor))

(event EventBeginPlay
  (Variables|Default|SetstartLocation (Transformation|GetActorLocation)))

(event Collision|EventActorBeginOverlap
  (params (OtherActor :type Actor%20Object%20Reference))
  (Utilities|Casting|CastToBP_2DSidescrollerCharacter OtherActor)
  (bind _location1 (Timeline|Timeline Play)
    (:Update
      (Transformation|SetActorLocation (+ _location1 (Variables|Default|GetstartLocation)) false false)
      (Utilities|Time|SetTimerbyEvent (delegate Custom|destroyPlatform) 0.1))))

(event EventTick
  (params (DeltaSeconds :type Float%20%28single-precision%29)))

(fn ConstructionScript)