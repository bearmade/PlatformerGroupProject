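; Tile map building actor that randomizes its appearance and spawns an enemy when play begins.
; BeginPlay randomly assigns one of the building tile maps to the render component.
; Every variant then spawns an AI pawn, picked at random from the first two Enemies entries, using the X and Z of the Scene component's world location.
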(event EventBeginPlay
  (bind _scene (Variables|Default|GetScene))
  (bind _returnvalue (Transformation|GetWorldLocation _scene))
  (|CallParentFunction)
  (switch int (Math|Random|RandomIntegerinRange 0 4)
    (:0
      (Class|PaperTileMapComponent|SetTileMap (Variables|Default|GetRenderComponent) "/Game/Tiles/ImportedTiles/Buildings/TM_Building_1.TM_Building_1"))
    (:1
      (Class|PaperTileMapComponent|SetTileMap (Variables|Default|GetRenderComponent) "/Game/Tiles/ImportedTiles/Buildings/TM_Building_2.TM_Building_2"))
    (:2
      (Class|PaperTileMapComponent|SetTileMap (Variables|Default|GetRenderComponent) "/Game/Tiles/ImportedTiles/Buildings/TM_Building_3.TM_Building_3"))
    (:3
      (Class|PaperTileMapComponent|SetTileMap (Variables|Default|GetRenderComponent) "/Game/Tiles/ImportedTiles/Buildings/TM_Building_4.TM_Building_4"))
    (:4
      (Class|PaperTileMapComponent|SetTileMap (Variables|Default|GetRenderComponent) "/Game/Tiles/ImportedTiles/Buildings/TM_Building_5.TM_Building_5")))
  (AI|SpawnAIFromClass (Utilities|Array|Get(acopy) (Variables|Default|GetEnemies) (Math|Random|RandomIntegerinRange 0 1)) 0 (Math|Vector|MakeVector (.x _returnvalue) 0.0 (.z _returnvalue)) "0, 0, 0" false 0))

(event Collision|EventActorBeginOverlap
  (params (OtherActor :type Actor%20Object%20Reference))
  (|CallParentFunction OtherActor) ; This node is disabled and will not be called.\nDrag off pins to build functionality.
)

(event EventTick
  (params (DeltaSeconds :type Float%20%28single-precision%29))
  (|CallParentFunction DeltaSeconds) ; This node is disabled and will not be called.\nDrag off pins to build functionality.
)

(fn ConstructionScript
  (|CallParentFunction))