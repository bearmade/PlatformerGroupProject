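; Water tile for the 2D sidescroller that lets the character swim and manages oxygen loss and drowning damage.
; Box overlap toggles swimming, gravity, jump limit and the HUD bubble bar.
; Self-looping Delays lower Oxygen while InWater after entry, but the exit loop also subtracts it while out of water.
; Tick applies slight damage whenever the player's Oxygen is depleted, regardless of overlap.
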(event OnComponentBeginOverlap(Box)
  (params (OverlappedComponent :type Primitive%20Component%20Object%20Reference) (OtherActor :type Actor%20Object%20Reference) (OtherComp :type Primitive%20Component%20Object%20Reference) (OtherBodyIndex :type Integer) (bFromSweep :type Boolean) (SweepResult :type Hit%20Result%20Structure%20%28by%20ref%29))
  (bind _asbp_2dsidescroller_character (Utilities|Casting|CastToBP_2DSidescrollerCharacter OtherActor))
  (Pawn|Components|CharacterMovement|SetMovementMode (Variables|/Script/Engine.Character|GetCharacterMovement _asbp_2dsidescroller_character) "MOVE_Swimming" 0)
  (Variables|/Script/Engine.CharacterMovementComponent|SetGravityScale (Variables|/Script/Engine.Character|GetCharacterMovement _asbp_2dsidescroller_character) 0.3)
  (Variables|/Game/Player/BP_2DSidescrollerCharacter.BP_2DSidescrollerCharacter_C|SetmaxJumps _asbp_2dsidescroller_character 1000)
  (Variables|Default|SetInWater true)
  (bind _foundwidgets (Widget|GetAllWidgetsOfClass "/Game/UI/WBP_WidgetHUD.WBP_WidgetHUD_C" true))
  (for _array_element _foundwidgets
    (Widget|SetVisibility (Variables|/Game/UI/WBP_WidgetHUD.WBP_WidgetHUD_C|GetBubbleBar _array_element) "Visible")
    (if (Variables|Default|GetInWater) :!label _label
      (bind _asbp_2dsidescroller_character_2 (Utilities|Casting|CastToBP_2DSidescrollerCharacter (Game|GetPlayerCharacter 0)))
      (Variables|/Game/Player/BP_2DSidescrollerCharacter.BP_2DSidescrollerCharacter_C|SetOxygen _asbp_2dsidescroller_character_2 (- (Variables|/Game/Player/BP_2DSidescrollerCharacter.BP_2DSidescrollerCharacter_C|GetOxygen _asbp_2dsidescroller_character_2) 1.0)))
    (Utilities|FlowControl|Delay 0.2)
    (goto _label)))

(event OnComponentEndOverlap(Box)
  (params (OverlappedComponent :type Primitive%20Component%20Object%20Reference) (OtherActor :type Actor%20Object%20Reference) (OtherComp :type Primitive%20Component%20Object%20Reference) (OtherBodyIndex :type Integer))
  (bind _asbp_2dsidescroller_character (Utilities|Casting|CastToBP_2DSidescrollerCharacter OtherActor))
  (Pawn|Components|CharacterMovement|SetMovementMode (Variables|/Script/Engine.Character|GetCharacterMovement _asbp_2dsidescroller_character) "MOVE_Falling" 0)
  (Variables|/Game/Player/BP_2DSidescrollerCharacter.BP_2DSidescrollerCharacter_C|SetmaxJumps _asbp_2dsidescroller_character 2)
  (Variables|/Script/Engine.CharacterMovementComponent|SetGravityScale (Variables|/Script/Engine.Character|GetCharacterMovement _asbp_2dsidescroller_character) 2.0)
  (Variables|Default|SetInWater false)
  (bind _foundwidgets (Widget|GetAllWidgetsOfClass "/Game/UI/WBP_WidgetHUD.WBP_WidgetHUD_C" true))
  (for _array_element _foundwidgets
    (Widget|SetVisibility (Variables|/Game/UI/WBP_WidgetHUD.WBP_WidgetHUD_C|GetBubbleBar _array_element) "Hidden")
    (if (Variables|Default|GetInWater) :!label _label
      _
      (else
        (bind _asbp_2dsidescroller_character_2 (Utilities|Casting|CastToBP_2DSidescrollerCharacter (Game|GetPlayerCharacter 0)))
        (Variables|/Game/Player/BP_2DSidescrollerCharacter.BP_2DSidescrollerCharacter_C|SetOxygen _asbp_2dsidescroller_character_2 (- (Variables|/Game/Player/BP_2DSidescrollerCharacter.BP_2DSidescrollerCharacter_C|GetOxygen _asbp_2dsidescroller_character_2) 1.0))))
    (Utilities|FlowControl|Delay 0.2)
    (goto _label)))

(event EventBeginPlay)

(event Collision|EventActorBeginOverlap
  (params (OtherActor :type Actor%20Object%20Reference)))

(event EventTick
  (params (DeltaSeconds :type Float%20%28single-precision%29))
  (bind _asbp_2dsidescroller_character (Utilities|Casting|CastToBP_2DSidescrollerCharacter (Game|GetPlayerCharacter 0)))
  (if (<= (Variables|/Game/Player/BP_2DSidescrollerCharacter.BP_2DSidescrollerCharacter_C|GetOxygen _asbp_2dsidescroller_character) 0.0)
    (Game|Damage|ApplyDamage _asbp_2dsidescroller_character 0.01 0 0)))

(fn ConstructionScript)