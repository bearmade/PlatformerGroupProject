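; BP_GroundPoundBlast is a short-lived blast actor, named for the player's ground pound, that destroys simple enemies it touches.
; It expires half a second after spawning.
; When its capsule overlaps a BP_SimpleEnemyFinal's capsule component, it destroys both that enemy and itself.
; On a hit, it spawns a brief PaperFlipbookActor at the hit location, calls SetFlipbook with no flipbook specified, then destroys itself.
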(event OnComponentBeginOverlap(Capsule)
  (params (OverlappedComponent :type Primitive%20Component%20Object%20Reference) (OtherActor :type Actor%20Object%20Reference) (OtherComp :type Primitive%20Component%20Object%20Reference) (OtherBodyIndex :type Integer) (bFromSweep :type Boolean) (SweepResult :type Hit%20Result%20Structure%20%28by%20ref%29))
  (bind _asbp_simple_enemy_final (Utilities|Casting|CastToBP_SimpleEnemyFinal OtherActor))
  (if (== (Variables|/Script/Engine.Character|GetCapsuleComponent _asbp_simple_enemy_final) OtherComp)
    (Actor|DestroyActor _asbp_simple_enemy_final)
    (Actor|DestroyActor)))

(event EventBeginPlay
  (Actor|SetLifeSpan 0.5))

(event Collision|EventActorBeginOverlap
  (params (OtherActor :type Actor%20Object%20Reference)))

(event EventTick
  (params (DeltaSeconds :type Float%20%28single-precision%29)))

(event Collision|EventHit
  (params (MyComp :type Primitive%20Component%20Object%20Reference) (Other :type Actor%20Object%20Reference) (OtherComp :type Primitive%20Component%20Object%20Reference) (bSelfMoved :type Boolean) (HitLocation :type Vector :default "0, 0, 0") (HitNormal :type Vector :default "0, 0, 0") (NormalImpulse :type Vector :default "0, 0, 0") (Hit :type Hit%20Result%20Structure%20%28by%20ref%29))
  (bind _returnvalue (Game|SpawnActorfromClass "/Script/Paper2D.PaperFlipbookActor" (Math|Conversions|ToTransform(Vector) HitLocation) "Undefined" "MultiplyWithRoot" 0 0))
  (Actor|SetLifeSpan _returnvalue 0.2)
  (Sprite|SetFlipbook (Variables|/Script/Paper2D.PaperFlipbookActor|GetRenderComponent _returnvalue))
  (Actor|DestroyActor))

(fn ConstructionScript)